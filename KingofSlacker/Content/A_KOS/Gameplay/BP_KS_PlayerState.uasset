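; Player state that holds the game's date, economy, KPI, fish energy, strive and inventory, and restores them from saved data.
; LoadGameSave moves the player character to the saved transform, copies date values into Task and stats into its variables, then passes item entries to InventoryComponent.
; Tick prints the day and month as debug text, plus a placeholder task message on every frame of day ten.
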(event EventBeginPlay)

(event EventTick
  (params (DeltaSeconds :type Float%20%28single-precision%29))
  (bind _task (Variables|Default|GetTask))
  (bind _day (Variables|/Script/KingofSlacker.TaskComponent|Getday _task))
  (Development|PrintString (Utilities|String|Append "day: " (Utilities|String|ToString(Integer) _day)) true true "(R=0.000000,G=0.660000,B=1.000000,A=1.000000)" DeltaSeconds)
  (Development|PrintString (Utilities|String|Append "month: " (Utilities|String|ToString(Integer) (Variables|/Script/KingofSlacker.TaskComponent|Getmonth _task))) true true "(R=0.000000,G=0.660000,B=1.000000,A=1.000000)" DeltaSeconds)
  (if (== _day 10)
    (Development|PrintString "Task1 happened")))

(fn ConstructionScript)

(fn LoadGameSave
  (params (LevelName :type String) (CharacterLocation :type Transform) (Time_Year :type Integer) (Time_Month :type Integer) (Time_Day :type Integer) (Money :type Integer) (Income :type Integer) (KPI :type Float%20%28double-precision%29) (KPI_Times :type Integer) (KPI_Count :type Float%20%28double-precision%29) (Fish_Energy :type Integer) (Fish_EnergyCount :type Integer) (Max_FishEnergy :type Integer) (StriveCurrent :type Float%20%28double-precision%29) (Slot_Name :type Array%20of%20Strings) (ItemEntries :type Array%20of%20Item%20Type%20Structures))
  (bind _returnvalue (Game|GetPlayerCharacter 0))
  (bind _task (Variables|Default|GetTask))
  (bind _asbp_test_character (Utilities|Casting|CastToBP_TestCharacter _returnvalue))
  (Utilities|IsValid _asbp_test_character
    (:Is%20Valid
      (Transformation|SetActorTransform _asbp_test_character CharacterLocation))
    (:Is%20Not%20Valid
      _))
  (Variables|/Script/KingofSlacker.TaskComponent|Setyear _task Time_Year)
  (Variables|/Script/KingofSlacker.TaskComponent|Setmonth _task Time_Month)
  (Variables|/Script/KingofSlacker.TaskComponent|Setday _task Time_Day)
  (Variables|Default|SetMoney Money)
  (Variables|Default|SetIncome Income)
  (Variables|Default|SetKPI KPI)
  (Variables|Default|SetKPITimes KPI_Times)
  (Variables|Default|SetKPICount KPI_Count)
  (Variables|Default|SetFish_Energy Fish_Energy)
  (Variables|Default|SetFish_Energy_Count Fish_EnergyCount)
  (Variables|Default|SetMaxFish_Energy Max_FishEnergy)
  (Variables|Default|SetStrive StriveCurrent)
  (Class|InventoryComponent|LoadItem (Variables|Default|GetInventoryComponent) ItemEntries))