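; Player controller that asks the game mode to spawn the player, creates the overlay widget and handles throw input.
; Throw input poses BP_TestCharacter and shows its arc, then release launches a BP_ParabolicPrediction actor by impulse; cancel aborts.
; It also holds timer-driven arc events that turn predicted projectile paths into spline meshes.
; Tick debug-prints player state attributes like money, KPI, energy and health; StartTask only prints.
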(event Custom|Draw%20Projectile%20Curve
  (bind _returnvalue (Utilities|Time|SetTimerbyEvent (delegate Custom|Update%20Projectile%20Curve) 0.1 true))
  (Variables|Default|SetProjectile%20Timer _returnvalue))

(event Custom|Update%20Projectile%20Curve
  (bind _projectile_spline (Variables|Default|GetProjectile%20Spline))
  (CallFunction|ClearSplinePoints)
  (bind _predictresult (Class|GameplayStatics|BlueprintPredictProjectilePathAdvanced (Utilities|Struct|MakePredictProjectilePathParams (Transformation|GetWorldLocation (Variables|Default|GetThrowable)) (+ (* (Variables|Default|GetThrow%20Force%20Forward) (Transformation|GetActorForwardVector)) (Math|Vector|MakeVector 0.0 0.0 (Variables|Default|GetThrow%20Force%20Up))) true 0.0 3.0 true "ECC_WorldStatic" "ObjectTypeQuery1" (Utilities|Array|MakeArray self) 2e+01 0.0 "None" 5.0 false)))
  (for _array_element (.PathData (Utilities|Struct|BreakPredictProjectilePathResult _predictresult))
    (Spline|AddSplinePoint (Variables|Default|GetProjectile%20Spline) (.Location (Utilities|Struct|BreakPredictProjectilePathPointData _array_element)) "World" true))
  (for _index (range 3 (Spline|GetNumberOfSplinePoints (Variables|Default|GetProjectile%20Spline)))
    (bind _returnvalue (AddComponent|AddSplineMeshComponent true))
    (Utilities|Array|Add (Variables|Default|GetSpline%20Mesh) _returnvalue)
    (SplineMesh|SetStartandEnd _returnvalue (.Location (Spline|GetLocationandTangentatSplinePoint _projectile_spline _index "World")) (.Tangent (Spline|GetLocationandTangentatSplinePoint _projectile_spline _index "World")) (Math|Vector|Lerp(Vector) (.Location (Spline|GetLocationandTangentatSplinePoint _projectile_spline _index "World")) (.Location (Spline|GetLocationandTangentatSplinePoint _projectile_spline (+ _index 1) "World")) 0.5) (Math|Vector|Lerp(Vector) (.Tangent (Spline|GetLocationandTangentatSplinePoint _projectile_spline _index "World")) (.Tangent (Spline|GetLocationandTangentatSplinePoint _projectile_spline (+ _index 1) "World")) 0.5) true :!class /Script/Engine.SplineMeshComponent)))

(event Custom|Clear%20Spline%20Points
  (bind _spline_mesh (Variables|Default|GetSpline%20Mesh))
  (Components|DestroyComponent _spline_mesh)
  (Utilities|Array|Clear _spline_mesh)
  (Spline|ClearSplinePoints (Variables|Default|GetProjectile%20Spline) true))

(event Input|EnhancedActionEvents|EnhancedInputActionIA_Throw
  (params (ActionValue :type Vector%202D%20Structure) (ElapsedSeconds :type Float%20%28double-precision%29) (TriggeredSeconds :type Float%20%28double-precision%29) (InputAction :type Input%20Action%20Object%20Reference :default "/Game/Input/Actions/IA_Throw.IA_Throw"))
  (:Ongoing
    (bind _asbp_test_character (Utilities|Casting|CastToBP_TestCharacter (Game|GetPlayerCharacter 0)))
    (bind _output_get (Variables|Default|SetBP_Player _asbp_test_character))
    (Components|StaticMesh|SetStaticMesh (Variables|/Game/A_KOS/Character/Player/BP_TestCharacter.BP_TestCharacter_C|GetThrowable _output_get) 0)
    (Default|DrawProjectileCurve (Variables|Default|GetBP_Player))
    (Animation|Montage|PlayMontage (Variables|/Script/Engine.Character|GetMesh _output_get) "/Game/A_KOS/Blueprints/Projectile/MF_Pistol_Idle_ADS_AO_CU_Montage.MF_Pistol_Idle_ADS_AO_CU_Montage" 0.0
      (:then
        (Variables|Default|SetReady%20To%20Throw true))))
  (:Completed
    (if (Variables|Default|GetReady%20To%20Throw)
      (Animation|StopAnimMontage (Variables|Default|GetBP_Player) "/Game/A_KOS/Blueprints/Projectile/MF_Pistol_Idle_ADS_AO_CU_Montage.MF_Pistol_Idle_ADS_AO_CU_Montage")
      (Utilities|Time|ClearandInvalidateTimerbyHandle (Variables|/Game/A_KOS/Character/Player/BP_TestCharacter.BP_TestCharacter_C|GetProjectile%20Timer (Variables|Default|GetBP_Player)))
      (Default|ClearSplinePoints (Variables|Default|GetBP_Player))
      (Components|StaticMesh|SetStaticMesh (Variables|/Game/A_KOS/Character/Player/BP_TestCharacter.BP_TestCharacter_C|GetThrowable (Variables|Default|GetBP_Player)) 0)
      (bind _returnvalue (Game|SpawnActorfromClass "/Game/A_KOS/Blueprints/Projectile/BP_ParabolicPrediction.BP_ParabolicPrediction_C" (Math|Transform|MakeTransform (Transformation|GetWorldLocation (Variables|/Game/A_KOS/Character/Player/BP_TestCharacter.BP_TestCharacter_C|GetThrowable (Variables|Default|GetBP_Player))) "0, 0, 0" "1.000000,1.000000,1.000000") "Undefined" "MultiplyWithRoot" (Variables|Default|GetBP_Player) 0))
      (Physics|AddImpulse (Variables|/Game/A_KOS/Blueprints/Projectile/BP_ParabolicPrediction.BP_ParabolicPrediction_C|GetProjectile _returnvalue) (+ (* (Variables|/Game/A_KOS/Character/Player/BP_TestCharacter.BP_TestCharacter_C|GetThrow%20Force%20Forward (Variables|Default|GetBP_Player)) (Transformation|GetActorForwardVector (Variables|Default|GetBP_Player))) (Math|Vector|MakeVector 0.0 0.0 (Variables|/Game/A_KOS/Character/Player/BP_TestCharacter.BP_TestCharacter_C|GetThrow%20Force%20Up (Variables|Default|GetBP_Player)))) "None" true)
      (Transformation|SetActorRotation (Pawn|GetControlRotation (Variables|Default|GetBP_Player) :!class /Script/Engine.Pawn)))))

(event Input|EnhancedActionEvents|EnhancedInputActionIA_CancelThrow
  (params (ActionValue :type Vector%202D%20Structure) (ElapsedSeconds :type Float%20%28double-precision%29) (TriggeredSeconds :type Float%20%28double-precision%29) (InputAction :type Input%20Action%20Object%20Reference :default "/Game/Input/Actions/IA_CancelThrow.IA_CancelThrow"))
  (:Started
    (Variables|Default|SetReady%20To%20Throw false)
    (Utilities|IsValid (Variables|Default|GetBP_Player)
      (:Is%20Valid
        (Default|ClearSplinePoints (Variables|Default|GetBP_Player))
        (Animation|StopAnimMontage (Variables|Default|GetBP_Player) "/Game/A_KOS/Blueprints/Projectile/MF_Pistol_Idle_ADS_AO_CU_Montage.MF_Pistol_Idle_ADS_AO_CU_Montage")))))

(event EventBeginPlay
  ;[0.15 0.15 0.15 0.5] 选择角色类型并开始游戏
  (Utilities|FlowControl|Sequence
    (:then_0
      (bind _asbp_ks_game_mode_base (Utilities|Casting|CastToBP_KS_GameModeBase (Game|GetGameMode)))
      (Default|SpawnPlayer _asbp_ks_game_mode_base self))
    (:then_1
      (bind _returnvalue (UserInterface|CreateWidget "/Game/A_KOS/UI/WBP_Overlay.WBP_Overlay_C"))
      (bind _output_get (Variables|Default|SetOverlay _returnvalue))
      (UserInterface|Viewport|AddtoViewport _output_get 0)
      (EventDispatchers|BindEventtoOnTaskRecived (Variables|Default|GetOverlay) (EventDispatchers|CreateEvent :!event StartTask)))))

(event EventTick
  (params (DeltaSeconds :type Float%20%28single-precision%29))
  (CallFunction|DEBUGPrintAllAttributes DeltaSeconds))

(fn ConstructionScript)

(fn DEBUGPrintAttribute
  (params (AttributeName :type String) (Input :type String) (Duration :type Float%20%28single-precision%29) (TextColor :type Linear%20Color%20Structure))
  (Development|PrintString (Utilities|String|Append AttributeName Input) true true TextColor Duration))

(fn DEBUGPrintAllAttributes
  (params (Duration :type Float%20%28single-precision%29))
  (bind _returnvalue (Class|KSPlayerController|GetKSPlayerState))
  (CallFunction|DEBUGPrintAttribute "Money : " (Utilities|String|ToString(Integer) (Variables|/Script/KingofSlacker.KS_PlayerState|GetMoney _returnvalue)) Duration "(R=0.987518,G=1.000000,B=0.000000,A=1.000000)")
  (CallFunction|DEBUGPrintAttribute "Income : " (Utilities|String|ToString(Integer) (Variables|/Script/KingofSlacker.KS_PlayerState|GetIncome _returnvalue)) Duration "(R=0.987518,G=1.000000,B=0.000000,A=1.000000)")
  (CallFunction|DEBUGPrintAttribute "KPI : " (Utilities|String|ToString(Float) (Variables|/Script/KingofSlacker.KS_PlayerState|GetKPI _returnvalue)) Duration "(R=0.987518,G=1.000000,B=0.000000,A=1.000000)")
  (CallFunction|DEBUGPrintAttribute "Max KPI : " (Utilities|String|ToString(Float) (Variables|/Script/KingofSlacker.KS_PlayerState|GetMaxKPI _returnvalue)) Duration "(R=0.987518,G=1.000000,B=0.000000,A=1.000000)")
  (CallFunction|DEBUGPrintAttribute "Fish Energy : " (Utilities|String|ToString(Integer) (Variables|/Script/KingofSlacker.KS_PlayerState|GetFish_Energy _returnvalue)) Duration "(R=0.000000,G=0.000000,B=1.000000,A=1.000000)")
  (CallFunction|DEBUGPrintAttribute "Max Fish Energy : " (Utilities|String|ToString(Integer) (Variables|/Script/KingofSlacker.KS_PlayerState|GetMaxFish_Energy _returnvalue)) Duration "(R=0.000000,G=0.000000,B=1.000000,A=1.000000)")
  (CallFunction|DEBUGPrintAttribute "Fish Effeciency : " (Utilities|String|ToString(Float) (Variables|/Script/KingofSlacker.KS_PlayerState|GetFish_EnergyEfficiency _returnvalue)) Duration "(R=0.000000,G=0.000000,B=1.000000,A=1.000000)")
  (CallFunction|DEBUGPrintAttribute "Fish Time" (Utilities|String|ToString(Float) (Variables|/Script/KingofSlacker.KS_PlayerState|GetFish_Time _returnvalue)) Duration "(R=0.000000,G=0.000000,B=1.000000,A=1.000000)")
  (CallFunction|DEBUGPrintAttribute "Strive : " (Utilities|String|ToString(Float) (Variables|/Script/KingofSlacker.KS_PlayerState|GetStrive _returnvalue)) Duration "(R=1.000000,G=0.000000,B=0.000000,A=1.000000)")
  (CallFunction|DEBUGPrintAttribute "Max Strive : " (Utilities|String|ToString(Float) (Variables|/Script/KingofSlacker.KS_PlayerState|GetMaxStrive _returnvalue)) Duration "(R=1.000000,G=0.000000,B=0.000000,A=1.000000)")
  (CallFunction|DEBUGPrintAttribute "Work Time : " (Utilities|String|ToString(Float) (Variables|/Script/KingofSlacker.KS_PlayerState|GetWork_Time _returnvalue)) Duration "(R=1.000000,G=0.000000,B=0.000000,A=1.000000)")
  (CallFunction|DEBUGPrintAttribute "Work Effciency ： " (Utilities|String|ToString(Float) (Variables|/Script/KingofSlacker.KS_PlayerState|GetWork_Efficiency _returnvalue)) Duration "(R=1.000000,G=0.000000,B=0.000000,A=1.000000)")
  (CallFunction|DEBUGPrintAttribute "Health : " (Utilities|String|ToString(Float) (Variables|/Script/KingofSlacker.KS_PlayerState|GetHealth _returnvalue)) Duration "(R=0.000000,G=1.000000,B=0.000000,A=1.000000)")
  (CallFunction|DEBUGPrintAttribute "MaxHealth : " (Utilities|String|ToString(Float) (Variables|/Script/KingofSlacker.KS_PlayerState|GetMaxHealth _returnvalue)) Duration "(R=0.000000,G=1.000000,B=0.000000,A=1.000000)"))

(fn StartTask
  (Development|PrintString "Start Task"))