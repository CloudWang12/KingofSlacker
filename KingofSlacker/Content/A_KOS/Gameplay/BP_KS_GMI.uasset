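; Game instance for King of Slacker that saves and loads game progress by slot name.
; SaveGame replaces any existing slot with a new SG_KingOfSlacker holding level, transform, date, player stats, inventory and cosmetic indices, filling FishEnergyCount from FishEnergy.
; LoadGame passes the saved data to the player state's LoadGameSave, omitting level name and cosmetics.
; Init caches player state and character one tick late, though saving and loading re-fetch player state.
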(event EventInit
  (Utilities|FlowControl|DelayUntilNextTick)
  (bind _asbp_ks_player_state (Utilities|Casting|CastToBP_KS_PlayerState (Game|GetPlayerState 0)))
  (Variables|Default|SetBP%20KS%20Player%20State _asbp_ks_player_state)
  (bind _asbp_test_character (Utilities|Casting|CastToBP_TestCharacter (Game|GetPlayerCharacter 0)))
  (Utilities|IsValid _asbp_test_character
    (:Is%20Valid
      (Variables|Default|SetPlayer _asbp_test_character))
    (:Is%20Not%20Valid
      (Development|PrintString "Character is not valid"))))

(fn SaveGame
  (params (SlotName :type String))
  (bind _returnvalue (Game|GetPlayerState 0))
  (bind _asbp_ks_player_state (Utilities|Casting|CastToBP_KS_PlayerState _returnvalue))
  (bind _returnvalue_2 (Actor|GetComponentbyClass _asbp_ks_player_state "/Script/KingofSlacker.TaskComponent"))
  (Variables|Default|SetSave%20Name SlotName)
  (bind _returnvalue_3 (SaveGame|DoesSaveGameExist (Variables|Default|GetSave%20Name)))
  (if _returnvalue_3
    (SaveGame|DeleteGameinSlot (Variables|Default|GetSave%20Name)))
  (bind _returnvalue_4 (Game|GetCurrentLevelName true))
  (bind _returnvalue_5 (SaveGame|CreateSaveGameObject "/Game/A_KOS/Blueprints/SaveGames/SG_KingOfSlacker.SG_KingOfSlacker_C"))
  (Variables|Default|SetBP%20KS%20Save%20Game _returnvalue_5)
  (Default|SetGameSave (Variables|Default|GetBP%20KS%20Save%20Game) _returnvalue_4 (Transformation|GetActorTransform (.AsBP%20Test%20Character (Utilities|Casting|CastToBP_TestCharacter (Game|GetPlayerCharacter 0)))) (Variables|/Script/KingofSlacker.TaskComponent|Getyear _returnvalue_2) (Variables|/Script/KingofSlacker.TaskComponent|Getmonth _returnvalue_2) (Variables|/Script/KingofSlacker.TaskComponent|Getday _returnvalue_2) (Variables|/Script/KingofSlacker.KS_PlayerState|GetMoney _asbp_ks_player_state) (Variables|/Script/KingofSlacker.KS_PlayerState|GetIncome _asbp_ks_player_state) (Variables|/Script/KingofSlacker.KS_PlayerState|GetKPI _asbp_ks_player_state) (Variables|/Script/KingofSlacker.KS_PlayerState|GetKPITimes _asbp_ks_player_state) (Variables|/Script/KingofSlacker.KS_PlayerState|GetKPICount _asbp_ks_player_state) (Variables|/Script/KingofSlacker.KS_PlayerState|GetFish_Energy _asbp_ks_player_state) (Variables|/Script/KingofSlacker.KS_PlayerState|GetFish_Energy _asbp_ks_player_state) (Variables|/Script/KingofSlacker.KS_PlayerState|GetMaxFish_Energy _asbp_ks_player_state) (Variables|/Script/KingofSlacker.KS_PlayerState|GetStrive _asbp_ks_player_state) 0 (Variables|/Script/KingofSlacker.InventoryComponent|GetItemEntries (Actor|GetComponentbyClass _asbp_ks_player_state "/Script/KingofSlacker.InventoryComponent")) (Variables|Default|GetCharacterSkinIndex) (Variables|Default|GetCharacterEmojiIndex) (Variables|Default|GetCharacterDecorationIdnex))
  (bind _returnvalue_6 (SaveGame|SaveGametoSlot (Variables|Default|GetBP%20KS%20Save%20Game) (Variables|Default|GetSave%20Name)))
  (if _returnvalue_6
    (Development|PrintString (Utilities|String|ToString(Boolean) _returnvalue_6))
    (Development|PrintString (Variables|Default|GetSave%20Name))))

(fn LoadGame
  (params (SlotName :type String))
  (bind _returnvalue (SaveGame|DoesSaveGameExist SlotName))
  (if _returnvalue
    (bind _returnvalue_2 (SaveGame|LoadGamefromSlot SlotName))
    (bind _assg_king_of_slacker (Utilities|Casting|CastToSG_KingOfSlacker _returnvalue_2))
    (Variables|Default|SetBP%20KS%20Save%20Game _assg_king_of_slacker)
    (Default|LoadGameSave (.AsBP%20KS%20Player%20State (Utilities|Casting|CastToBP_KS_PlayerState (Game|GetPlayerState 0))) "" (Variables|/Game/A_KOS/Blueprints/SaveGames/SG_KingOfSlacker.SG_KingOfSlacker_C|GetCharacterLocation (Variables|Default|GetBP%20KS%20Save%20Game)) (Variables|/Game/A_KOS/Blueprints/SaveGames/SG_KingOfSlacker.SG_KingOfSlacker_C|GetTime_Year (Variables|Default|GetBP%20KS%20Save%20Game)) (Variables|/Game/A_KOS/Blueprints/SaveGames/SG_KingOfSlacker.SG_KingOfSlacker_C|GetTime_Month (Variables|Default|GetBP%20KS%20Save%20Game)) (Variables|/Game/A_KOS/Blueprints/SaveGames/SG_KingOfSlacker.SG_KingOfSlacker_C|GetTime_Day (Variables|Default|GetBP%20KS%20Save%20Game)) (Variables|/Game/A_KOS/Blueprints/SaveGames/SG_KingOfSlacker.SG_KingOfSlacker_C|GetMoney (Variables|Default|GetBP%20KS%20Save%20Game)) (Variables|/Game/A_KOS/Blueprints/SaveGames/SG_KingOfSlacker.SG_KingOfSlacker_C|GetIncome (Variables|Default|GetBP%20KS%20Save%20Game)) (Variables|/Game/A_KOS/Blueprints/SaveGames/SG_KingOfSlacker.SG_KingOfSlacker_C|GetKPI (Variables|Default|GetBP%20KS%20Save%20Game)) (Variables|/Game/A_KOS/Blueprints/SaveGames/SG_KingOfSlacker.SG_KingOfSlacker_C|GetKPI_Times (Variables|Default|GetBP%20KS%20Save%20Game)) (Variables|/Game/A_KOS/Blueprints/SaveGames/SG_KingOfSlacker.SG_KingOfSlacker_C|GetKPI_Count (Variables|Default|GetBP%20KS%20Save%20Game)) (Variables|/Game/A_KOS/Blueprints/SaveGames/SG_KingOfSlacker.SG_KingOfSlacker_C|GetFish_Energy (Variables|Default|GetBP%20KS%20Save%20Game)) (Variables|/Game/A_KOS/Blueprints/SaveGames/SG_KingOfSlacker.SG_KingOfSlacker_C|GetFish_EnergyCount (Variables|Default|GetBP%20KS%20Save%20Game)) (Variables|/Game/A_KOS/Blueprints/SaveGames/SG_KingOfSlacker.SG_KingOfSlacker_C|GetMax_FishEnergy (Variables|Default|GetBP%20KS%20Save%20Game)) (Variables|/Game/A_KOS/Blueprints/SaveGames/SG_KingOfSlacker.SG_KingOfSlacker_C|GetStrive (Variables|Default|GetBP%20KS%20Save%20Game)) (Variables|/Game/A_KOS/Blueprints/SaveGames/SG_KingOfSlacker.SG_KingOfSlacker_C|GetSlotName (Variables|Default|GetBP%20KS%20Save%20Game)) (Variables|/Game/A_KOS/Blueprints/SaveGames/SG_KingOfSlacker.SG_KingOfSlacker_C|GetItemEntries (Variables|Default|GetBP%20KS%20Save%20Game)))
    (Development|PrintString "游戏已读取")))