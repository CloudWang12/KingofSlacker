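; Character selection stage that acts as the view target, opens the main menu and previews the player's cosmetic customization.
; The menu's left and right button events drive category switches that step through skins, face emojis and decorations.
; Choices update the mesh material, expression widget or decoration mesh, and save their indices to BP_KS_GMI.
; Hat functions exist, but neither category switch calls them.
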(event EventBeginPlay
  (bind _returnvalue (Game|GetPlayerController 0))
  (Utilities|FlowControl|Sequence
    (:then_0
      (bind _asbp_ks_gmi (Utilities|Casting|CastToBP_KS_GMI (Game|GetGameInstance)))
      (Variables|Default|SetAs%20BP%20KS%20GMI _asbp_ks_gmi)
      (Input|SetInputModeUIOnly _returnvalue 0 "DoNotLock" false)
      (Variables|/Script/Engine.PlayerController|SetbShowMouseCursor _returnvalue true)
      (Game|Player|SetViewTargetwithBlend _returnvalue self 0.0 "VTBlend_Linear" 0.0 false)
      (bind _returnvalue_2 (UserInterface|CreateWidget "/Game/A_KOS/UI/MainMenu/WBP_MainMenu.WBP_MainMenu_C" _returnvalue))
      (Variables|Default|SetWBP_MainMenu _returnvalue_2)
      (UserInterface|Viewport|AddtoViewport _returnvalue_2 0)
      (bind _aswbp_face_expression (Utilities|Casting|CastToWBP_FaceExpression (UserInterface|GetUserWidgetObject (Variables|Default|GetExpressionComponent))))
      (Variables|Default|SetAs%20WBP%20Face%20Expression _aswbp_face_expression))
    (:then_1
      (EventDispatchers|BindEventtoOnButtonLeftClicked (Variables|/Game/A_KOS/UI/MainMenu/WBP_MainMenu.WBP_MainMenu_C|GetWBP_CharacterChoose (Variables|Default|GetWBP_MainMenu)) (EventDispatchers|CreateEvent :!event SwitchFunctionLeftClicked))
      (EventDispatchers|BindEventtoOnButtonRightClicked (Variables|/Game/A_KOS/UI/MainMenu/WBP_MainMenu.WBP_MainMenu_C|GetWBP_CharacterChoose (Variables|Default|GetWBP_MainMenu)) (EventDispatchers|CreateEvent :!event SwitchFunctionRightClicked))
      (Emoji|SetCharacterEmoji))))

(fn ConstructionScript
  (Skin|SetCharacterSkin))

(fn NextCharacterSkin
  (Utilities|IsValid (Variables|Default|GetAs%20BP%20KS%20GMI)
    (:Is%20Valid
      (bind _result (Math|Integer|IncrementInt (Variables|Default|GetSkinIndex))
        (:%20%20
          (bind _output_get (Variables|Default|SetSkinIndex (Math|Integer|Clamp(Integer) _result 0 (- (Utilities|Array|Length (Variables|Default|GetCharacterSkin)) 1))))
          (Variables|/Game/A_KOS/Gameplay/BP_KS_GMI.BP_KS_GMI_C|SetCharacterSkinIndex (Variables|Default|GetAs%20BP%20KS%20GMI) _output_get)
          (Skin|SetCharacterSkin))))))

(fn PreCharacterSkin
  (Utilities|IsValid (Variables|Default|GetAs%20BP%20KS%20GMI)
    (:Is%20Valid
      (bind _result (Math|Integer|DecrementInt (Variables|Default|GetSkinIndex))
        (:%20%20
          (bind _output_get (Variables|Default|SetSkinIndex (Math|Integer|Clamp(Integer) _result 0 (- (Utilities|Array|Length (Variables|Default|GetCharacterSkin)) 1))))
          (Variables|/Game/A_KOS/Gameplay/BP_KS_GMI.BP_KS_GMI_C|SetCharacterSkinIndex (Variables|Default|GetAs%20BP%20KS%20GMI) _output_get)
          (Skin|SetCharacterSkin))))))

(fn SetCharacterSkin
  (Rendering|Material|SetMaterial (Variables|Default|GetSkeletalMesh) 0 (Utilities|Array|Get(acopy) (Variables|Default|GetCharacterSkin) (Variables|Default|GetSkinIndex))))

(fn PreCharacterHats
  (Utilities|IsValid (Variables|Default|GetAs%20BP%20KS%20GMI)
    (:Is%20Valid
      (bind _result (Math|Integer|DecrementInt (Variables|Default|GetHatIndex))
        (:%20%20
          (bind _output_get (Variables|Default|SetHatIndex (Math|Integer|Clamp(Integer) _result 0 (Utilities|Array|Length (Variables|Default|GetCharacterHats)))))
          (Variables|/Game/A_KOS/Gameplay/BP_KS_GMI.BP_KS_GMI_C|SetCharacterHatIndex (Variables|Default|GetAs%20BP%20KS%20GMI) _output_get)
          (Hat|SetCharacterHat))))))

(fn NextCharacterHats
  (Utilities|IsValid (Variables|Default|GetAs%20BP%20KS%20GMI)
    (:Is%20Valid
      (bind _result (Math|Integer|IncrementInt (Variables|Default|GetHatIndex))
        (:%20%20
          (bind _output_get (Variables|Default|SetHatIndex _result))
          (Variables|/Game/A_KOS/Gameplay/BP_KS_GMI.BP_KS_GMI_C|SetCharacterHatIndex (Variables|Default|GetAs%20BP%20KS%20GMI) (Math|Integer|Clamp(Integer) _output_get 0 (- (Utilities|Array|Length (Variables|Default|GetCharacterHats)) 1)))
          (Hat|SetCharacterHat))))))

(fn PreCharacterEmoji
  (Utilities|IsValid (Variables|Default|GetAs%20BP%20KS%20GMI)
    (:Is%20Valid
      (bind _result (Math|Integer|DecrementInt (Variables|Default|GetEmojiIndex))
        (:%20%20
          (bind _output_get (Variables|Default|SetEmojiIndex (Math|Integer|Clamp(Integer) _result 0 (- (Utilities|Array|Length (Variables|Default|GetCharacterEmoji)) 1))))
          (Variables|/Game/A_KOS/Gameplay/BP_KS_GMI.BP_KS_GMI_C|SetCharacterEmojiIndex (Variables|Default|GetAs%20BP%20KS%20GMI) _output_get)
          (Emoji|SetCharacterEmoji))))))

(fn NextCharacterEmoji
  (Utilities|IsValid (Variables|Default|GetAs%20BP%20KS%20GMI)
    (:Is%20Valid
      (bind _result (Math|Integer|IncrementInt (Variables|Default|GetEmojiIndex))
        (:%20%20
          (bind _output_get (Variables|Default|SetEmojiIndex (Math|Integer|Clamp(Integer) _result 0 (- (Utilities|Array|Length (Variables|Default|GetCharacterEmoji)) 1))))
          (Variables|/Game/A_KOS/Gameplay/BP_KS_GMI.BP_KS_GMI_C|SetCharacterEmojiIndex (Variables|Default|GetAs%20BP%20KS%20GMI) _output_get)
          (Emoji|SetCharacterEmoji))))))

(fn PreCharacterDecoration
  (Utilities|IsValid (Variables|Default|GetAs%20BP%20KS%20GMI)
    (:Is%20Valid
      (bind _result (Math|Integer|DecrementInt (Variables|Default|GetDecorationIndex))
        (:%20%20
          (bind _output_get (Variables|Default|SetDecorationIndex (Math|Integer|Clamp(Integer) _result 0 (- (Utilities|Array|Length (Variables|Default|GetCharacterDecoration)) 1))))
          (Variables|/Game/A_KOS/Gameplay/BP_KS_GMI.BP_KS_GMI_C|SetCharacterDecorationIdnex (Variables|Default|GetAs%20BP%20KS%20GMI) _output_get)
          (Decoration|SetCharacterDecoration))))))

(fn SetCharacterDecoration
  (Components|StaticMesh|SetStaticMesh (Variables|Default|GetDecoration) (Utilities|Array|Get(acopy) (Variables|Default|GetCharacterDecoration) (Variables|Default|GetDecorationIndex))))

(fn NextCharacterDecoration
  (Utilities|IsValid (Variables|Default|GetAs%20BP%20KS%20GMI)
    (:Is%20Valid
      (bind _result (Math|Integer|IncrementInt (Variables|Default|GetDecorationIndex))
        (:%20%20
          (bind _output_get (Variables|Default|SetDecorationIndex (Math|Integer|Clamp(Integer) _result 0 (- (Utilities|Array|Length (Variables|Default|GetCharacterDecoration)) 1))))
          (Variables|/Game/A_KOS/Gameplay/BP_KS_GMI.BP_KS_GMI_C|SetCharacterDecorationIdnex (Variables|Default|GetAs%20BP%20KS%20GMI) _output_get)
          (Decoration|SetCharacterDecoration))))))

(fn SetCharacterHat
  (Components|StaticMesh|SetStaticMesh (Variables|Default|GetHat) (Utilities|Array|Get(acopy) (Variables|Default|GetCharacterHats) (Variables|Default|GetHatIndex))))

(fn SetCharacterEmoji
  (Default|UpdateExpressionBrush (Variables|Default|GetAs%20WBP%20Face%20Expression) (Utilities|Array|Get(acopy) (Variables|Default|GetCharacterEmoji) (Variables|Default|GetEmojiIndex))))

(fn SwitchFunctionLeftClicked
  (params (CategoryIndex :type Integer))
  (switch int CategoryIndex
    (:1
      (Skin|PreCharacterSkin))
    (:2
      (Emoji|PreCharacterEmoji))
    (:3
      (Decoration|PreCharacterDecoration))))

(fn SwitchFunctionRightClicked
  (params (CategoryIndex :type Integer))
  (switch int CategoryIndex
    (:1
      (Skin|NextCharacterSkin))
    (:2
      (Emoji|NextCharacterEmoji))
    (:3
      (Decoration|NextCharacterDecoration))))