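; BP_ItemActorBase is a base actor for inventory items, carrying an ItemType with name, description and quantity.
; Its Interact event enables or disables the actor's input for player controller 0 based on the InRange flag.
; While input is enabled, IA_Interact prints a test string and the item's fields through DEBUGItemInformation, with no pickup logic.
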(event Input|EnhancedActionEvents|EnhancedInputActionIA_Interact
  (params (ActionValue :type Boolean) (ElapsedSeconds :type Float%20%28double-precision%29) (TriggeredSeconds :type Float%20%28double-precision%29) (InputAction :type Input%20Action%20Object%20Reference :default "/Game/Input/Actions/IA_Interact.IA_Interact"))
  (:Started
    (Development|PrintString "Hello")
    (CallFunction|DEBUGItemInformation)))

(event EventBeginPlay)

(event Collision|EventActorBeginOverlap
  (params (OtherActor :type Actor%20Object%20Reference)))

(event EventTick
  (params (DeltaSeconds :type Float%20%28single-precision%29)))

(event EventInteract
  (params (bInRange :type Boolean))
  (bind _returnvalue (Game|GetPlayerController 0))
  (if bInRange
    (Input|EnableInput _returnvalue)
    (else
      (Input|DisableInput _returnvalue))))

(fn ConstructionScript)

(fn DEBUGItemInformation
  (bind _itemtype (Variables|Default|GetItemType))
  (bind (_itemname _itemdescription _itemquantity) (Utilities|Struct|BreakItemType _itemtype))
  (Development|PrintString (Utilities|String|ToString(Text) _itemname))
  (Development|PrintString (Utilities|String|ToString(Text) _itemdescription))
  (Development|PrintString (Utilities|String|ToString(Integer) _itemquantity)))