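; Work desk interactable where the player holds Space to work, with rewards in strive, KPI and money through OnStriveAdd.
; Interact toggles input and operation guides by range, showing a content tip once.
; Working snaps the character to the seat, disables movement and changes expression and player status; release restores them.
; Desk item events reveal or swap props by item ID, and Tick turns the progress bar toward the camera.
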(event Custom|SwitchDesktop
  (params (ItemType :type Item%20Type%20Structure))
  (CallFunction|UpdateDeskSetup (.ItemID (Utilities|Struct|BreakItemType ItemType))))

(event Input|EnhancedActionEvents|EnhancedInputActionIA_Space
  (params (ActionValue :type Boolean) (ElapsedSeconds :type Float%20%28double-precision%29) (TriggeredSeconds :type Float%20%28double-precision%29) (InputAction :type Input%20Action%20Object%20Reference :default "/Game/Input/Actions/IA_Space.IA_Space"))
  (bind _as_bp_ks_player_state (Variables|Default|GetAs%20BP%20KS%20Player%20State))
  (bind _bp_player (Variables|Default|GetBP%20Player))
  (bind _bp_player_2 (Variables|Default|GetBP%20Player))
  (bind _bp_player_3 (Variables|Default|GetBP%20Player))
  (bind _charactermovement (Variables|/Script/Engine.Character|GetCharacterMovement _bp_player_3))
  (:Ongoing
    (if (Utilities|Enum|Equal(Enum) (Variables|/Game/A_KOS/Gameplay/BP_KS_PlayerState.BP_KS_PlayerState_C|GetPlayerStatus (Variables|Default|GetAs%20BP%20KS%20Player%20State)) "Station_Idle")
      (Default|HideOperationGuide _bp_player_2)
      (Class|StationBase|OnSpacePressed)
      (Default|UpdateExpression _bp_player (.OutItem (Utilities|Array|Random (Utilities|Array|MakeArray "/Game/A_KOS/Asset/main_charactor/charactor_material/EMOJI/WORK_EMO1.WORK_EMO1" "/Game/A_KOS/Asset/main_charactor/charactor_material/EMOJI/WORK_EMO2.WORK_EMO2"))))
      (Variables|/Game/A_KOS/Gameplay/BP_KS_PlayerState.BP_KS_PlayerState_C|SetPlayerStatus _as_bp_ks_player_state "Station_Working")
      (Variables|Default|SetPlayerTransformBeforeWork (Transformation|GetWorldTransform (Variables|/Script/Engine.Actor|GetRootComponent _bp_player_3)))
      (Transformation|SetActorRelativeTransform _bp_player_3 (Transformation|GetWorldTransform (Variables|Default|GetPlayerPosition)) false false)
      (Components|Activation|SetActive _charactermovement false false)))
  (:Canceled
    (if (Utilities|Enum|Equal(Enum) (Variables|/Game/A_KOS/Gameplay/BP_KS_PlayerState.BP_KS_PlayerState_C|GetPlayerStatus (Variables|Default|GetAs%20BP%20KS%20Player%20State)) "Station_Working") :!label _label
      (Default|ShowOperationGuide _bp_player_2 1)
      (Class|StationBase|OnSpaceReleased)
      (Default|UpdateExpression _bp_player (.OutItem (Utilities|Array|Random (Utilities|Array|MakeArray "/Game/A_KOS/Asset/main_charactor/charactor_material/EMOJI/main_normal1.main_normal1" "/Game/A_KOS/Asset/main_charactor/charactor_material/EMOJI/main_normal2.main_normal2"))))
      (Variables|/Game/A_KOS/Gameplay/BP_KS_PlayerState.BP_KS_PlayerState_C|SetPlayerStatus _as_bp_ks_player_state "Station_Idle")
      (Transformation|SetActorRelativeTransform _bp_player_3 (Variables|Default|GetPlayerTransformBeforeWork) false false)
      (Components|Activation|SetActive _charactermovement true false)))
  (:Completed
    (goto _label)))

(event EventTick
  (params (DeltaSeconds :type Float%20%28single-precision%29))
  (CallFunction|UpdateTipsWidget))

(event EventInteract
  (params (bInRange :type Boolean))
  (bind _returnvalue (Game|GetPlayerController 0))
  (Variables|Default|SetbInRange bInRange)
  (bind _asbp_character_base (Utilities|Casting|CastToBP_Character_Base (Game|GetPlayerCharacter 0))
    (:then
      (Variables|Default|SetBP%20Player _asbp_character_base))
    (:CastFailed
      _))
  (if bInRange
    (Utilities|FlowControl|Sequence
      (:then_0
        (Utilities|FlowControl|DoOnce false
          (:Completed
            (Default|OpenContentTips (Variables|/Game/A_KOS/Gameplay/BP_KS_PlayerController.BP_KS_PlayerController_C|GetOverlay (Variables|Default|GetAs%20BP%20KS%20Player%20Controller)) 3))))
      (:then_1
        (Input|EnableInput _returnvalue)
        (Default|ShowOperationGuide (Variables|Default|GetBP%20Player) 1)))
    (else
      (Input|DisableInput _returnvalue)
      (Default|HideOperationGuide (Variables|Default|GetBP%20Player) 1))))

(event EventBeginPlay
  (Utilities|FlowControl|Sequence
    (:then_0
      (EventDispatchers|BindEventtoOnBarProgressMax (EventDispatchers|CreateEvent :!event OnStriveAdd))
      (bind _asbp_ks_player_controller (Utilities|Casting|CastToBP_KS_PlayerController (Game|GetPlayerController 0)))
      (bind _output_get (Variables|Default|SetAs%20BP%20KS%20Player%20Controller _asbp_ks_player_controller))
      (Utilities|IsValid _output_get
        (:Is%20Valid
          (bind _asbp_ks_player_state (Utilities|Casting|CastToBP_KS_PlayerState (Game|GetPlayerState 0)))
          (Variables|Default|SetAs%20BP%20KS%20Player%20State _asbp_ks_player_state)
          (Utilities|IsValid _asbp_ks_player_state
            (:Is%20Valid
              (Variables|Default|SetEffectTimes (Variables|/Script/KingofSlacker.KS_PlayerState|GetWork_Time _asbp_ks_player_state)))))))
    (:then_1
      (EventDispatchers|BindEventtoOnDeskItemShow (Variables|Default|GetAs%20BP%20KS%20Player%20Controller) (EventDispatchers|CreateEvent :!event Custom|SwitchDesktop)))))

(fn ConstructionScript)

(fn OnStriveAdd
  (bind _as_bp_ks_player_state (Variables|Default|GetAs%20BP%20KS%20Player%20State))
  (Class|KSPlayerState|AddUpStrive _as_bp_ks_player_state)
  (Class|KSPlayerState|AddupKPI _as_bp_ks_player_state)
  (Class|KSPlayerState|AddUpMoney _as_bp_ks_player_state 20))

(fn UpdateDeskSetup
  (params (Index :type Integer))
  (switch int Index
    (:1
      (Rendering|SetVisibility (Variables|Default|GetDrinking) true false))
    (:2
      (Rendering|SetVisibility (Variables|Default|GetToilet) true false))
    (:3
      (Rendering|SetVisibility (Variables|Default|Getkeyboard0) false false)
      (Rendering|SetVisibility (Variables|Default|Getkeyboard1) true false))
    (:4
      (Rendering|SetVisibility (Variables|Default|GetMouse0) false false)
      (Rendering|SetVisibility (Variables|Default|GetMouse1) true false))
    (:5
      (Rendering|SetVisibility (Variables|Default|GetScreen0) false false)
      (Rendering|SetVisibility (Variables|Default|GetScreen1) true false))))

(fn UpdateTipsWidget
  (bind _progressbar (Variables|Default|GetProgressBar))
  (Transformation|SetWorldRotation _progressbar (Math|Rotator|FindLookatRotation (Transformation|GetWorldLocation _progressbar) (Transformation|GetActorLocation (Game|GetPlayerCameraManager 0))) false false))

(fn GetItemActorRef
  (return 0))

(fn GetItemIncome
  (return 0))

(fn GetItemName
  (return ""))

(fn GetName
  (return ""))

(fn GetTexture
  (return 0))