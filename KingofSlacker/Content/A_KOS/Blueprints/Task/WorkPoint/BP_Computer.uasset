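; Computer work point where the player holds Space in range to work; its strive handler raises the player's Strive and KPI.
; Interact toggles input by range, and BeginPlay binds the progress-bar-max event and takes EffectTimes from the player state's WorkTime.
; Holding switches status to working, changes expression, snaps the character to PlayerPosition and deactivates movement.
; Releasing or canceling restores idle status, a normal expression, the saved transform and movement.
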(event Input|EnhancedActionEvents|EnhancedInputActionIA_Space
  (params (ActionValue :type Boolean) (ElapsedSeconds :type Float%20%28double-precision%29) (TriggeredSeconds :type Float%20%28double-precision%29) (InputAction :type Input%20Action%20Object%20Reference :default "/Game/Input/Actions/IA_Space.IA_Space"))
  (bind _as_bp_ks_player_state (Variables|Default|GetAs%20BP%20KS%20Player%20State))
  (bind _as_bp_test_character (Variables|Default|GetAs%20BP%20Test%20Character))
  (bind _as_bp_test_character_2 (Variables|Default|GetAs%20BP%20Test%20Character))
  (bind _charactermovement (Variables|/Script/Engine.Character|GetCharacterMovement _as_bp_test_character_2))
  (:Ongoing
    (if (Utilities|Enum|Equal(Enum) (Variables|/Game/A_KOS/Gameplay/BP_KS_PlayerState.BP_KS_PlayerState_C|GetPlayerStatus (Variables|Default|GetAs%20BP%20KS%20Player%20State)) "Station_Idle")
      (Class|StationBase|OnSpacePressed)
      (Default|UpdateExpression _as_bp_test_character (.OutItem (Utilities|Array|Random (Utilities|Array|MakeArray "/Game/A_KOS/Asset/main_charactor/charactor_material/EMOJI/WORK_EMO1.WORK_EMO1" "/Game/A_KOS/Asset/main_charactor/charactor_material/EMOJI/WORK_EMO2.WORK_EMO2"))))
      (Variables|/Game/A_KOS/Gameplay/BP_KS_PlayerState.BP_KS_PlayerState_C|SetPlayerStatus _as_bp_ks_player_state "Station_Working")
      (Variables|Default|SetPlayerTransformBeforeWork (Transformation|GetWorldTransform (Variables|/Script/Engine.Actor|GetRootComponent _as_bp_test_character_2)))
      (Transformation|SetActorRelativeTransform _as_bp_test_character_2 (Transformation|GetWorldTransform (Variables|Default|GetPlayerPosition)) false false)
      (Components|Activation|SetActive _charactermovement false false)))
  (:Canceled
    (if (Utilities|Enum|Equal(Enum) (Variables|/Game/A_KOS/Gameplay/BP_KS_PlayerState.BP_KS_PlayerState_C|GetPlayerStatus (Variables|Default|GetAs%20BP%20KS%20Player%20State)) "Station_Working") :!label _label
      (Class|StationBase|OnSpaceReleased)
      (Default|UpdateExpression _as_bp_test_character (.OutItem (Utilities|Array|Random (Utilities|Array|MakeArray "/Game/A_KOS/Asset/main_charactor/charactor_material/EMOJI/main_normal1.main_normal1" "/Game/A_KOS/Asset/main_charactor/charactor_material/EMOJI/main_normal2.main_normal2"))))
      (Variables|/Game/A_KOS/Gameplay/BP_KS_PlayerState.BP_KS_PlayerState_C|SetPlayerStatus _as_bp_ks_player_state "Station_Idle")
      (Transformation|SetActorRelativeTransform _as_bp_test_character_2 (Variables|Default|GetPlayerTransformBeforeWork) false false)
      (Components|Activation|SetActive _charactermovement true false)))
  (:Completed
    (goto _label)))

(event Collision|EventActorBeginOverlap
  (params (OtherActor :type Actor%20Object%20Reference)))

(event EventInteract
  (params (bInRange :type Boolean))
  (bind _returnvalue (Game|GetPlayerController 0))
  (Variables|Default|SetbInRange bInRange)
  (bind _asbp_character_base (Utilities|Casting|CastToBP_Character_Base (Game|GetPlayerCharacter 0))
    (:then
      (Variables|Default|SetAs%20BP%20Test%20Character _asbp_character_base))
    (:CastFailed
      _))
  (if bInRange
    (Input|EnableInput _returnvalue)
    (else
      (Input|DisableInput _returnvalue))))

(event EventBeginPlay
  (EventDispatchers|BindEventtoOnBarProgressMax (EventDispatchers|CreateEvent :!event OnStriveAdd))
  (bind _asbp_ks_player_state (Utilities|Casting|CastToBP_KS_PlayerState (Game|GetPlayerState 0)))
  (Variables|Default|SetAs%20BP%20KS%20Player%20State _asbp_ks_player_state)
  (Utilities|IsValid _asbp_ks_player_state
    (:Is%20Valid
      (Variables|Default|SetEffectTimes (Variables|/Script/KingofSlacker.KS_PlayerState|GetWork_Time _asbp_ks_player_state)))))

(fn ConstructionScript)

(fn OnStriveAdd
  (bind _as_bp_ks_player_state (Variables|Default|GetAs%20BP%20KS%20Player%20State))
  (Class|KSPlayerState|AddUpStrive _as_bp_ks_player_state)
  (Class|KSPlayerState|AddupKPI _as_bp_ks_player_state))

(fn GetItemActorRef
  (return 0))

(fn GetItemIncome
  (return 0))

(fn GetItemName
  (return ""))

(fn GetName
  (return ""))

(fn GetTexture
  (return 0))