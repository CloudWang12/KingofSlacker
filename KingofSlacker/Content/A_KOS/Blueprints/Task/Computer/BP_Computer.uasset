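; BP_Computer is an interactable computer actor with a screen widget, driven by the Space key.
; Interact enables or disables player input on the actor according to whether the player is in range.
; Space press and release call OnSpacePressed and OnSpaceReleased.
; BeginPlay caches the WBP_Computer from the widget component, and Tick prints BarValue on screen as debug output.
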(event EventBeginPlay
  (bind _aswbp_computer (Utilities|Casting|CastToWBP_Computer (UserInterface|GetWidget (Variables|Default|GetWidget))))
  (Variables|Default|SetAs%20WBP%20Computer _aswbp_computer))

(event Collision|EventActorBeginOverlap
  (params (OtherActor :type Actor%20Object%20Reference)))

(event EventTick
  (params (DeltaSeconds :type Float%20%28single-precision%29))
  (Development|PrintString (Utilities|String|ToString(Float) (Variables|Default|GetBarValue)) true true "(R=0.000000,G=0.660000,B=1.000000,A=1.000000)" DeltaSeconds))

(event EventInteract
  (params (bInRange :type Boolean))
  (bind _returnvalue (Game|GetPlayerController 0))
  (Variables|Default|SetbInRange bInRange)
  (if bInRange
    (Input|EnableInput _returnvalue)
    (else
      (Input|DisableInput _returnvalue))))

(event Input|KeyboardEvents|SpaceBar
  (params (Key :type Key%20Structure :default "None"))
  (:Pressed
    (Class|StationBase|OnSpacePressed))
  (:Released
    (Class|StationBase|OnSpaceReleased)))

(fn ConstructionScript)