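; Fish pool interactable that serves as a task, toggling player input and an operation guide as the player enters or leaves range.
; On BeginPlay it binds a handler to the progress-bar-max event and copies FishTime from the player state into EffectTimes.
; OnFishEnergyChanged adds fish energy and lowers Strive on the player state.
; The item getters are empty stubs.
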(event EventBeginPlay
  (EventDispatchers|BindEventtoOnBarProgressMax (EventDispatchers|CreateEvent :!event OnFishEnergyChanged))
  (bind _asbp_ks_player_state (Utilities|Casting|CastToBP_KS_PlayerState (Game|GetPlayerState 0)))
  (Variables|Default|SetAs%20BP%20KS%20Player%20State _asbp_ks_player_state)
  (Utilities|IsValid _asbp_ks_player_state
    (:Is%20Valid
      (Variables|Default|SetEffectTimes (Variables|/Script/KingofSlacker.KS_PlayerState|GetFish_Time _asbp_ks_player_state)))))

(event Collision|EventActorBeginOverlap
  (params (OtherActor :type Actor%20Object%20Reference)))

(event EventTick
  (params (DeltaSeconds :type Float%20%28single-precision%29)))

(event EventInteract
  (params (bInRange :type Boolean))
  (bind _returnvalue (Game|GetPlayerController 0))
  (bind _output_get (Variables|Default|SetbInRange bInRange))
  (bind _asbp_character_base (Utilities|Casting|CastToBP_Character_Base (Game|GetPlayerCharacter 0))
    (:then
      (Variables|Default|SetBP%20Player _asbp_character_base))
    (:CastFailed
      _))
  (if _output_get
    (Input|EnableInput _returnvalue)
    (Default|ShowOperationGuide (Variables|Default|GetBP%20Player) 1)
    (else
      (Input|DisableInput _returnvalue)
      (Default|HideOperationGuide (Variables|Default|GetBP%20Player) 1))))

(fn ConstructionScript)

(fn OnFishEnergyChanged
  (bind _as_bp_ks_player_state (Variables|Default|GetAs%20BP%20KS%20Player%20State))
  (Class|KSPlayerState|AddUpFishEnergy _as_bp_ks_player_state)
  (Class|KSPlayerState|LowDownStrive _as_bp_ks_player_state 10))

(fn GetItemActorRef
  (return 0))

(fn GetItemIncome
  (return 0))

(fn GetItemName
  (return ""))

(fn GetName
  (return ""))

(fn GetTexture
  (return 0))