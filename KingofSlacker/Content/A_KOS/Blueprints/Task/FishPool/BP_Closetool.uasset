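; Closetool station in the FishPool task set, where the player holds Space to "fish" with a phone shown.
; While held from StationIdle, it switches to StationFishing, saves the player's transform, snaps them to PlayerPosition and deactivates movement.
; Releasing or canceling restores transform, movement and idle status, and hides the phone.
; Both transitions update the operation guide, fishing type and a randomly picked expression, with player-state checks preventing repeat triggers.
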(event Input|EnhancedActionEvents|EnhancedInputActionIA_Space
  (params (ActionValue :type Boolean) (ElapsedSeconds :type Float%20%28double-precision%29) (TriggeredSeconds :type Float%20%28double-precision%29) (InputAction :type Input%20Action%20Object%20Reference :default "/Game/Input/Actions/IA_Space.IA_Space"))
  (bind _bp_player (Variables|Default|GetBP%20Player))
  (bind _as_bp_ks_player_state (Variables|Default|GetAs%20BP%20KS%20Player%20State))
  (bind _bp_player_2 (Variables|Default|GetBP%20Player))
  (bind _bp_player_3 (Variables|Default|GetBP%20Player))
  (bind _phoneposition (Variables|/Game/A_KOS/Character/Player/BP_Character_Base.BP_Character_Base_C|GetPhonePosition _bp_player))
  (bind _charactermovement (Variables|/Script/Engine.Character|GetCharacterMovement _bp_player))
  (:Ongoing
    (if (Utilities|Enum|Equal(Enum) (Variables|/Game/A_KOS/Gameplay/BP_KS_PlayerState.BP_KS_PlayerState_C|GetPlayerStatus (Variables|Default|GetAs%20BP%20KS%20Player%20State)) "Station_Idle")
      (Default|HideOperationGuide _bp_player_3 1)
      (Class|StationBase|OnSpacePressed)
      (Variables|/Game/A_KOS/Character/Player/BP_Character_Base.BP_Character_Base_C|SetFishingType _bp_player_2 "NewEnumerator1")
      (Default|UpdateExpression _bp_player_2 (.OutItem (Utilities|Array|Random (Utilities|Array|MakeArray "/Game/A_KOS/Asset/main_charactor/charactor_material/EMOJI/WC_EMO1.WC_EMO1" "/Game/A_KOS/Asset/main_charactor/charactor_material/EMOJI/WC_EMO2.WC_EMO2"))))
      (Class|KSPlayerState|SwitchStatus _as_bp_ks_player_state "Station_Fishing")
      (Rendering|SetVisibility _phoneposition true false)
      (Variables|Default|SetPlayerTransformBeforeWork (Transformation|GetWorldTransform (Variables|/Script/Engine.Character|GetCapsuleComponent _bp_player)))
      (Transformation|SetActorRelativeTransform _bp_player (Transformation|GetWorldTransform (Variables|Default|GetPlayerPosition)) false false)
      (Components|Activation|SetActive _charactermovement false false)))
  (:Canceled
    (if (Utilities|Enum|Equal(Enum) (Variables|/Game/A_KOS/Gameplay/BP_KS_PlayerState.BP_KS_PlayerState_C|GetPlayerStatus (Variables|Default|GetAs%20BP%20KS%20Player%20State)) "Station_Fishing") :!label _label
      (Default|ShowOperationGuide _bp_player_3 1)
      (Class|StationBase|OnSpaceReleased)
      (Variables|/Game/A_KOS/Character/Player/BP_Character_Base.BP_Character_Base_C|SetFishingType _bp_player_2 "NewEnumerator2")
      (Default|UpdateExpression _bp_player_2 (.OutItem (Utilities|Array|Random (Utilities|Array|MakeArray "/Game/A_KOS/Asset/main_charactor/charactor_material/EMOJI/main_normal1.main_normal1" "/Game/A_KOS/Asset/main_charactor/charactor_material/EMOJI/main_normal2.main_normal2"))))
      (Class|KSPlayerState|SwitchStatus _as_bp_ks_player_state "Station_Idle")
      (Rendering|SetVisibility _phoneposition false false)
      (Transformation|SetActorRelativeTransform _bp_player (Variables|Default|GetPlayerTransformBeforeWork) false false)
      (Components|Activation|SetActive _charactermovement true false)))
  (:Completed
    (goto _label)))

(event EventBeginPlay
  (|CallParentFunction) ; 此节点被禁用，将不会被调用。\n从引脚连出引线来编译功能。
)

(event Collision|EventActorBeginOverlap
  (params (OtherActor :type Actor%20Object%20Reference))
  (|CallParentFunction OtherActor) ; 此节点被禁用，将不会被调用。\n从引脚连出引线来编译功能。
)

(event EventTick
  (params (DeltaSeconds :type Float%20%28single-precision%29))
  (|CallParentFunction DeltaSeconds) ; 此节点被禁用，将不会被调用。\n从引脚连出引线来编译功能。
)

(fn ConstructionScript
  (|CallParentFunction))