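; Chat NPC that the player talks to by holding Space while in range.
; Interact toggles input and the operation guide by range.
; Holding Space turns both characters face to face, reuses the StationFishing status, disables player movement, sets a random player talk expression, and runs a timeline stepping the NPC face widget through talk expressions.
; Releasing or canceling stops the timeline and restores idle status, movement and expressions.
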(event Input|EnhancedActionEvents|EnhancedInputActionIA_Space
  (params (ActionValue :type Boolean) (ElapsedSeconds :type Float%20%28double-precision%29) (TriggeredSeconds :type Float%20%28double-precision%29) (InputAction :type Input%20Action%20Object%20Reference :default "/Game/Input/Actions/IA_Space.IA_Space"))
  (bind _as_bp_ks_player_state (Variables|Default|GetAs%20BP%20KS%20Player%20State))
  (bind _bp_player (Variables|Default|GetBP%20Player))
  (bind _skeletalmesh (Variables|Default|GetSkeletalMesh))
  (bind _bp_player_2 (Variables|Default|GetBP%20Player))
  (bind _wbp_face_expression_npc (Variables|Default|GetWBP%20Face%20Expression%20Npc))
  (bind _bp_player_3 (Variables|Default|GetBP%20Player))
  (bind _bp_player_4 (Variables|Default|GetBP%20Player))
  (bind _charactermovement (Variables|/Script/Engine.Character|GetCharacterMovement _bp_player))
  (:Ongoing
    (if (Utilities|Enum|Equal(Enum) (Variables|/Game/A_KOS/Gameplay/BP_KS_PlayerState.BP_KS_PlayerState_C|GetPlayerStatus (Variables|Default|GetAs%20BP%20KS%20Player%20State)) "Station_Idle")
      (Default|HideOperationGuide _bp_player_4 1)
      (Class|StationBase|OnSpacePressed)
      (Variables|/Game/A_KOS/Character/Player/BP_Character_Base.BP_Character_Base_C|SetFishingType _bp_player_3 "NewEnumerator3")
      (Default|UpdateExpression _bp_player_3 (.OutItem (Utilities|Array|Random (Utilities|Array|MakeArray "/Game/A_KOS/Asset/main_charactor/charactor_material/EMOJI/talk_emo2_01.talk_emo2_01" "/Game/A_KOS/Asset/main_charactor/charactor_material/EMOJI/talk_emo1_01.talk_emo1_01"))))
      (Transformation|SetActorRotation _bp_player_2 (Math|Rotator|MakeRotator 0.0 0.0 (.yaw (Math|Rotator|FindLookatRotation (Transformation|GetActorLocation _bp_player_2) (Transformation|GetWorldLocation (Variables|Default|GetSkeletalMesh))))))
      (Transformation|SetRelativeRotation _skeletalmesh (Math|Rotator|MakeRotator 0.0 0.0 (+ (.yaw (Math|Rotator|FindLookatRotation (Transformation|GetWorldLocation _skeletalmesh) (Transformation|GetActorLocation (Variables|Default|GetBP%20Player)))) 9e+01)) false false)
      (Class|KSPlayerState|SwitchStatus _as_bp_ks_player_state "Station_Fishing")
      (Components|Activation|SetActive _charactermovement false false)
      (bind _expressionchange (Timeline|时间轴_0 Play)
        (:Update
          (if (< _expressionchange 1.0)
            (Default|UpdateExpressionBrush _wbp_face_expression_npc "/Game/A_KOS/Asset/main_charactor/charactor_material/EMOJI/talk_emo1_01.talk_emo1_01")
            (elif (< _expressionchange 2.0)
              (Default|UpdateExpressionBrush _wbp_face_expression_npc "/Game/A_KOS/Asset/main_charactor/charactor_material/EMOJI/talk_emo1_02.talk_emo1_02")
              (elif (< _expressionchange 3.0)
                (Default|UpdateExpressionBrush _wbp_face_expression_npc "/Game/A_KOS/Asset/main_charactor/charactor_material/EMOJI/talk_emo2_01.talk_emo2_01")
                (elif (< _expressionchange 4.0)
                  (Default|UpdateExpressionBrush _wbp_face_expression_npc "/Game/A_KOS/Asset/main_charactor/charactor_material/EMOJI/talk_emo2_02.talk_emo2_02")))))))))
  (:Canceled
    (if (Utilities|Enum|Equal(Enum) (Variables|/Game/A_KOS/Gameplay/BP_KS_PlayerState.BP_KS_PlayerState_C|GetPlayerStatus (Variables|Default|GetAs%20BP%20KS%20Player%20State)) "Station_Fishing") :!label _label
      (Default|ShowOperationGuide _bp_player_4 1)
      (Class|StationBase|OnSpaceReleased)
      (Variables|/Game/A_KOS/Character/Player/BP_Character_Base.BP_Character_Base_C|SetFishingType _bp_player_3 "NewEnumerator2")
      (Default|UpdateExpression _bp_player_3 (.OutItem (Utilities|Array|Random (Utilities|Array|MakeArray "/Game/A_KOS/Asset/main_charactor/charactor_material/EMOJI/main_normal1.main_normal1" "/Game/A_KOS/Asset/main_charactor/charactor_material/EMOJI/main_normal2.main_normal2"))))
      (Utilities|FlowControl|Sequence
        (:then_0
          (Timeline|时间轴_0 Stop))
        (:then_1
          (Class|KSPlayerState|SwitchStatus _as_bp_ks_player_state "Station_Idle")
          (Components|Activation|SetActive _charactermovement true false)
          (Default|UpdateExpressionBrush (Variables|Default|GetWBP%20Face%20Expression%20Npc) "/Game/A_KOS/Asset/main_charactor/charactor_material/EMOJI/talk_emo1_02.talk_emo1_02")))))
  (:Completed
    (goto _label)))

(event EventBeginPlay
  (|CallParentFunction)
  (bind _aswbp_face_expression_npc (Utilities|Casting|CastToWBP_FaceExpression_Npc (UserInterface|GetUserWidgetObject (Variables|Default|GetExpressionComponent))))
  (Variables|Default|SetWBP%20Face%20Expression%20Npc _aswbp_face_expression_npc))

(event Collision|EventActorBeginOverlap
  (params (OtherActor :type Actor%20Object%20Reference))
  (|CallParentFunction OtherActor) ; 此节点被禁用，将不会被调用。\n从引脚连出引线来编译功能。
)

(event EventTick
  (params (DeltaSeconds :type Float%20%28single-precision%29))
  (|CallParentFunction DeltaSeconds) ; 此节点被禁用，将不会被调用。\n从引脚连出引线来编译功能。
)

(event EventInteract
  (params (bInRange :type Boolean))
  (bind _returnvalue (Game|GetPlayerController 0))
  (bind _output_get (Variables|Default|SetbInRange bInRange))
  (bind _asbp_character_base (Utilities|Casting|CastToBP_Character_Base (Game|GetPlayerCharacter 0))
    (:then
      (Variables|Default|SetBP%20Player _asbp_character_base))
    (:CastFailed
      _))
  (if _output_get
    (Input|EnableInput _returnvalue)
    (Default|ShowOperationGuide (Variables|Default|GetBP%20Player) 1)
    (else
      (Input|DisableInput _returnvalue)
      (Default|HideOperationGuide (Variables|Default|GetBP%20Player) 1))))

(fn ConstructionScript
  (|CallParentFunction))

(fn UpdateExpression
  (params (Expression :type Texture%202D%20Object%20Reference) (SkinMaterial :type Material%20Interface%20Object%20Reference)))