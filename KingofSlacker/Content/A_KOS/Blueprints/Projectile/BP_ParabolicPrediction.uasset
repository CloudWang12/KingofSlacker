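; Projectile actor that shows its predicted impact point in flight and infects NPCs it hits.
; Each tick it predicts the path from the projectile's current position and velocity, moving an impact marker, revealed shortly after spawn, to the predicted hit.
; On hit it spawns a burst effect and destroys itself, after a short delay for non-NPCs.
; NPC hits apply infection, report and apply damage credited to the player, and set the blackboard hurt flag.
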(event OnComponentHit(Projectile)
  (params (HitComponent :type Primitive%20Component%20Object%20Reference) (OtherActor :type Actor%20Object%20Reference) (OtherComp :type Primitive%20Component%20Object%20Reference) (NormalImpulse :type Vector :default "0, 0, 0") (Hit :type Hit%20Result%20Structure%20%28by%20ref%29))
  (bind _returnvalue (Game|GetPlayerCharacter 0))
  (bind _asbp_npc_base (Utilities|Casting|CastToBP_NPC_Base OtherActor)
    (:then
      (Variables|Default|SetBP%20NPC _asbp_npc_base))
    (:CastFailed
      (Utilities|FlowControl|Delay 1.0)))
  (Niagara|SpawnSystematLocation "/Niagara/DefaultAssets/Templates/Systems/DirectionalBurstLightweight.DirectionalBurstLightweight" (Transformation|GetWorldLocation (Variables|Default|GetProjectile)) "0, 0, 0" "3.000000,3.000000,1.000000" true true "AutoRelease")
  (Utilities|IsValid (Variables|Default|GetBP%20NPC)
    (:Is%20Valid
      (Default|Infection (Variables|Default|GetBP%20NPC) (Variables|Default|GetDamage))
      (Default|ChangeInfectionValue (Variables|Default|GetBP%20NPC))
      (Class|AISenseDamage|ReportDamageEvent (Variables|Default|GetBP%20NPC) _returnvalue 1.0 (Transformation|GetActorLocation _returnvalue) "0, 0, 0" "None")
      (Game|Damage|ApplyDamage (Variables|Default|GetBP%20NPC) 1.0 0 _returnvalue)
      (AI|Components|Blackboard|SetValueasBool (AI|GetBlackboard (Variables|Default|GetBP%20NPC)) (Utilities|Name|MakeLiteralName "bHurt") true))
    (:Is%20Not%20Valid
      _))
  (Actor|DestroyActor))

(event EventBeginPlay
  (Utilities|FlowControl|Delay 0.25)
  (Development|SetHiddeninGame (Variables|Default|GetImpact%20Point%20Prediction) false false))

(event Collision|EventActorBeginOverlap
  (params (OtherActor :type Actor%20Object%20Reference)))

(event EventTick
  (params (DeltaSeconds :type Float%20%28single-precision%29))
  (bind _projectile (Variables|Default|GetProjectile))
  (bind _predictresult (Class|GameplayStatics|BlueprintPredictProjectilePathAdvanced (Utilities|Struct|MakePredictProjectilePathParams (Transformation|GetWorldLocation _projectile) (Transformation|GetComponentVelocity _projectile) true 1.0 1.0 true "ECC_WorldStatic" "ObjectTypeQuery1" (Utilities|Array|MakeArray self))))
  (for (_array_element _array_index) (.PathData (Utilities|Struct|BreakPredictProjectilePathResult _predictresult))
    (if (== _array_index 0)
      (Variables|Default|SetLastLocation (.Location (Utilities|Struct|BreakPredictProjectilePathPointData _array_element)))))
  (Transformation|SetWorldLocation (Variables|Default|GetImpact%20Point%20Prediction) (.Location (Collision|BreakHitResult (.HitResult (Utilities|Struct|BreakPredictProjectilePathResult _predictresult)))) false false))

(fn ConstructionScript)