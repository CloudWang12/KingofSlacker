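; SG_KingOfSlacker is a save-game object for King of Slacker that holds a snapshot of player progress.
; It stores level and location, in-game date, money and income, KPI, fish energy, strive, inventory items, character cosmetics and the slot name.
; A single SetGameSave function copies all these values from its inputs into the matching variables, with no disk save or load logic in this graph.
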(fn SetGameSave
  (params (LevelName :type String) (CharacterLocation :type Transform) (Time_Year :type Integer) (Time_Month :type Integer) (Time_Day :type Integer) (Money :type Integer) (Income :type Integer) (KPI :type Float%20%28double-precision%29) (KPI_Times :type Integer) (KPI_Count :type Float%20%28double-precision%29) (Fish_Energy :type Integer) (Fish_EnergyCount :type Integer) (Max_FishEnergy :type Integer) (Strive :type Float%20%28double-precision%29) (SlotName :type String) (ItemEntries :type Array%20of%20Item%20Type%20Structures) (CharacterSkinIndex :type Integer) (CharacterEmojiIndex :type Integer) (CharacterDecorationIndex :type Integer))
  (Variables|Default|SetLevelName LevelName)
  (Variables|Default|SetCharacterLocation CharacterLocation)
  (Variables|Default|SetTime_Year Time_Year)
  (Variables|Default|SetTime_Month Time_Month)
  (Variables|Default|SetTime_Day Time_Day)
  (Variables|Default|SetMoney Money)
  (Variables|Default|SetIncome Income)
  (Variables|Default|SetKPI KPI)
  (Variables|Default|SetKPI_Times KPI_Times)
  (Variables|Default|SetKPI_Count KPI_Count)
  (Variables|Default|SetFish_Energy Fish_Energy)
  (Variables|Default|SetFish_EnergyCount Fish_EnergyCount)
  (Variables|Default|SetMax_FishEnergy Max_FishEnergy)
  (Variables|Default|SetStrive Strive)
  (Variables|Default|SetSlotName SlotName)
  (Variables|Default|SetItemEntries ItemEntries)
  (Variables|Default|SetCharacterSkinIndex CharacterSkinIndex)
  (Variables|Default|SetCharacterEmojiIndex CharacterEmojiIndex)
  (Variables|Default|SetCharacterDecorationIndex CharacterDecorationIndex))