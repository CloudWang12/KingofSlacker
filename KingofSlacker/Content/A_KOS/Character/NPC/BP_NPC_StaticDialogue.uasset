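; NPC actor that plays linear dialogue from DT_NPCDialogue, keyed by NPCName, when an in-range player in StationIdle interacts.
; A looping timeline cycles talk expressions on the face widget and advances lines, then restores a random default expression and hides the dialogue.
; The name widget turns toward the camera every tick.
; Talking gates interaction but is never set true here; the item getters are empty stubs.
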(event EventBeginPlay
  (CallFunction|ExpressionComponentInit)
  (bind _asbp_ks_player_state (Utilities|Casting|CastToBP_KS_PlayerState (Game|GetPlayerState 0)))
  (Variables|Default|SetAs%20BP%20KS%20Player%20State _asbp_ks_player_state)
  (bind _aswbp_npcname (Utilities|Casting|CastToWBP_NPCName (UserInterface|GetUserWidgetObject (Variables|Default|GetName))))
  (Default|UpdateName _aswbp_npcname (Utilities|Text|ToText(Name) (Variables|Default|GetNPCName)))
  (bind _aswbp_npcdialogue (Utilities|Casting|CastToWBP_NPCDialogue (UserInterface|GetUserWidgetObject (Variables|Default|GetDialogue))))
  (Variables|Default|SetAs%20WBP%20NPCDialogue _aswbp_npcdialogue))

(event Collision|EventActorBeginOverlap
  (params (OtherActor :type Actor%20Object%20Reference)))

(event EventTick
  (params (DeltaSeconds :type Float%20%28single-precision%29))
  (CallFunction|UpdateTipsWidget))

(event EventInteract
  (params (bInRange :type Boolean))
  (if (Math|Boolean|ANDBoolean (Utilities|Enum|Equal(Enum) (Variables|/Game/A_KOS/Gameplay/BP_KS_PlayerState.BP_KS_PlayerState_C|GetPlayerStatus (Variables|Default|GetAs%20BP%20KS%20Player%20State)) "Station_Idle") (not (Variables|Default|GetbTalking)) bInRange)
    (bind _returnvalue (Utilities|GetDataTableRow "/Game/A_KOS/Character/NPC/Data/DT_NPCDialogue.DT_NPCDialogue" (Variables|Default|GetNPCName))
      (:then
        (Default|UpdateDialogue (Variables|Default|GetAs%20WBP%20NPCDialogue) (Utilities|Array|Get(acopy) (Utilities|Struct|BreakS_NPCDialogue _returnvalue)))
        (Rendering|SetVisibility (Variables|Default|GetDialogue) true false)
        (bind _expressionchange (Timeline|时间轴 PlayFromStart)
          (:Update
            (if (< _expressionchange 1.0)
              (CallFunction|UpdateExpression "/Game/A_KOS/Asset/main_charactor/charactor_material/EMOJI/talk_emo1_01.talk_emo1_01" "/Game/A_KOS/Asset/main_charactor/charactor_material/M_Skin_NPC.M_Skin_NPC")
              (elif (< _expressionchange 2.0)
                (CallFunction|UpdateExpression "/Game/A_KOS/Asset/main_charactor/charactor_material/EMOJI/talk_emo1_02.talk_emo1_02" "/Game/A_KOS/Asset/main_charactor/charactor_material/M_Skin_NPC.M_Skin_NPC")
                (elif (< _expressionchange 3.0)
                  (CallFunction|UpdateExpression "/Game/A_KOS/Asset/main_charactor/charactor_material/EMOJI/talk_emo2_01.talk_emo2_01" "/Game/A_KOS/Asset/main_charactor/charactor_material/M_Skin_NPC.M_Skin_NPC")
                  (elif (< _expressionchange 4.0)
                    (CallFunction|UpdateExpression "/Game/A_KOS/Asset/main_charactor/charactor_material/EMOJI/talk_emo2_02.talk_emo2_02" "/Game/A_KOS/Asset/main_charactor/charactor_material/M_Skin_NPC.M_Skin_NPC"))))))
          (:Finished
            (Default|UpdateDialogue (Variables|Default|GetAs%20WBP%20NPCDialogue) (Utilities|Array|Get(acopy) (Utilities|Struct|BreakS_NPCDialogue _returnvalue) (Variables|Default|GetRounds)))
            (Math|Integer|IncrementInt (Variables|Default|GetRounds)
              (:%20%20
                (if (< (Variables|Default|GetRounds) (+ (Utilities|Array|Length (Utilities|Struct|BreakS_NPCDialogue _returnvalue)) 1))
                  (Timeline|时间轴 PlayFromStart)
                  (else
                    (Development|PrintString "3")
                    (Variables|Default|SetbTalking false)
                    (CallFunction|UpdateExpression (.OutItem (Utilities|Array|Random (Variables|Default|GetDefault%20Expression))) "/Game/A_KOS/Asset/main_charactor/charactor_material/M_Skin_NPC.M_Skin_NPC")
                    (Rendering|SetVisibility (Variables|Default|GetDialogue) false false)
                    (Variables|Default|SetRounds 1)))))))))))

(fn ConstructionScript)

(fn UpdateTipsWidget
  (bind _name (Variables|Default|GetName))
  (Transformation|SetWorldRotation _name (Math|Rotator|FindLookatRotation (Transformation|GetWorldLocation _name) (Transformation|GetActorLocation (Game|GetPlayerCameraManager 0))) false false))

(fn UpdateExpression
  (params (Expression :type Texture%202D%20Object%20Reference) (SkinMaterial :type Material%20Interface%20Object%20Reference))
  (Default|UpdateExpressionBrush (Variables|Default|GetWBP%20Face%20Expression%20Npc) Expression)
  (Rendering|Material|SetMaterial (Variables|Character|GetMesh) 0 SkinMaterial))

(fn ExpressionComponentInit
  (bind _aswbp_face_expression_npc (Utilities|Casting|CastToWBP_FaceExpression_Npc (UserInterface|GetUserWidgetObject (Variables|Default|GetExpressionComponent))))
  (bind _output_get (Variables|Default|SetWBP%20Face%20Expression%20Npc _aswbp_face_expression_npc))
  (Default|UpdateExpressionBrush _output_get (.OutItem (Utilities|Array|Random (Variables|Default|GetDefault%20Expression)))))

(fn GetItemActorRef
  (return 0))

(fn GetItemIncome
  (return 0))

(fn GetItemName
  (return ""))

(fn GetName
  (return ""))

(fn GetTexture
  (return 0))