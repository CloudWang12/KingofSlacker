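; Base NPC that tracks an alert level against the player and can be temporarily infected by projectile damage.
; When the blackboard flags an encountered player, the alert bar fills and, at full, broadcasts a report and has the player's overlay trigger arrest; otherwise it drains by the player's HideSpeed.
; Reaching maximum infection increments the player's infection count; infection replaces detection with a countdown that resets on expiry.
; Widget components show expressions, camera-facing bars and timed speech bubbles.
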(event Custom|UpdateDetectionProgress
  ;[0 0 0 0.5 36] 警告进度条逻辑
  (if (and (== (Variables|Patrol|GetAlertProgress) 0.0) (not (Variables|Patrol|GetbInGracePeriod)))
    (Alert|AlertProgressBarReset)
    (elif (ScalableFloat|GetValueasBool (AI|GetBlackboard 0) (Utilities|Name|MakeLiteralName "bEncounteredPlayer"))
      (Alert|AlertLevelRising)
      (if (== (Variables|Patrol|GetAlertProgress) 1.0)
        (Utilities|FlowControl|DoOnce false :!label _label
          (:Completed
            (Default|CallBroadcastNPCReport)
            (bind _asbp_ks_player_controller (Utilities|Casting|CastToBP_KS_PlayerController (Game|GetPlayerController 0)))
            (Utilities|IsValid (Variables|/Game/A_KOS/Gameplay/BP_KS_PlayerController.BP_KS_PlayerController_C|GetOverlay _asbp_ks_player_controller)
              (:Is%20Valid
                (Default|BeArrest (Variables|/Game/A_KOS/Gameplay/BP_KS_PlayerController.BP_KS_PlayerController_C|GetOverlay _asbp_ks_player_controller)))))))
      (else
        (Alert|AlertValueDrops)
        (goto _label Reset)))))

(event EventBeginPlay
  (CallFunction|ExpressionComponentInit)
  (CallFunction|InfectionProgressBarInit)
  (CallFunction|AlertProgressBarInit)
  (bind _aswbp_npcbubble (Utilities|Casting|CastToWBP_NPCBubble (UserInterface|GetUserWidgetObject (Variables|Default|GetBubble))))
  (Variables|Default|SetWBP%20NPCBubble _aswbp_npcbubble)
  (bind _output_get (Variables|Default|SetRandomDuration (Math|Random|RandomFloatinRange 3.0 1e+01)))
  (bind _returnvalue (Utilities|Time|SetTimerbyEvent (EventDispatchers|CreateEvent :!event UpdateBubble) _output_get true))
  (Variables|Default|SetBubbleTimer _returnvalue))

(event Collision|EventActorBeginOverlap
  (params (OtherActor :type Actor%20Object%20Reference)))

(event EventTick
  (params (DeltaSeconds :type Float%20%28single-precision%29))
  (CallFunction|DEBUGALL DeltaSeconds)
  (CallFunction|UpdateTipsWidget)
  (if (Variables|Default|GetbInfection)
    (CallFunction|CountdowntotheEndOfInfection DeltaSeconds)
    (else
      (CallFunction|UpdateDetectionProgress))))

(event Game|Damage|EventAnyDamage
  (params (Damage :type Float%20%28single-precision%29) (DamageType :type Damage%20Type%20Object%20Reference) (InstigatedBy :type Controller%20Object%20Reference) (DamageCauser :type Actor%20Object%20Reference))
  (CallFunction|UpdateExpression (Variables|Expression|GetConfused%20Expression) (Variables|Expression|GetConfused%20Skin))
  (Utilities|FlowControl|DoOnce false :!label _label
    (:Completed
      (Utilities|FlowControl|Delay 3.0)
      (CallFunction|UpdateExpression (.OutItem (Utilities|Array|Random (Variables|Expression|GetDefault%20Expression))) (Variables|Expression|GetDefault%20Skin))
      (goto _label Reset))))

(fn ConstructionScript)

(fn DEBUG
  (params (Append :type String) (Context :type String) (TextColor :type Linear%20Color%20Structure) (Duration :type Float%20%28single-precision%29))
  (Development|PrintString (Utilities|String|Append Append Context) true true TextColor Duration))

(fn DEBUGALL
  (params (Duration :type Float%20%28single-precision%29)))

(fn Infection
  (params (Projectile%20damage :type Integer))
  (bind _returnvalue (Game|GetPlayerController 0))
  (bind _asbp_ks_player_controller (Utilities|Casting|CastToBP_KS_PlayerController _returnvalue))
  (bind _bp_ks_player_state (Variables|/Game/A_KOS/Gameplay/BP_KS_PlayerController.BP_KS_PlayerController_C|GetBP%20KS%20Player%20State _asbp_ks_player_controller))
  (if (< (Variables|Infection|GetInfection%20Value) (Variables|Infection|GetMax%20Infection%20Value))
    (if (< (+ Projectile%20damage (Variables|Infection|GetInfection%20Value)) (Variables|Infection|GetMax%20Infection%20Value))
      (Variables|Infection|SetInfection%20Value (+ Projectile%20damage (Variables|Infection|GetInfection%20Value)))
      (Development|PrintString (Utilities|String|Append "NPC:" (Utilities|GetDisplayName self) "的感染值:" (Utilities|String|ToString(Integer) (Variables|Infection|GetInfection%20Value))))
      (else
        (Variables|Infection|SetInfection%20Value (Variables|Infection|GetMax%20Infection%20Value) :!label _label)
        (Variables|Default|SetbInfection true)
        (Development|PrintString (Utilities|String|Append "NPC:" (Utilities|GetDisplayName self) "已被感染"))
        (bind _result (Math|Integer|IncrementInt (Variables|/Script/KingofSlacker.KS_PlayerState|GetInfectionCount _bp_ks_player_state))
          (:%20%20
            (Variables|/Script/KingofSlacker.KS_PlayerState|SetInfectionCount _bp_ks_player_state _result)))))
    (else
      (goto _label))))

(fn ChangeInfectionValue
  (bind _wbp_point_prgress (Variables|Default|GetWBP%20Point%20Prgress))
  (switch int (Variables|Infection|GetInfection%20Value)
    (:0
      (Default|Reset _wbp_point_prgress))
    (:1
      (Default|UpdatePoint1 _wbp_point_prgress))
    (:2
      (Default|UpdatePoint2 _wbp_point_prgress))
    (:3
      (Default|UpdatePoint3 _wbp_point_prgress))
    (:4
      (Default|UpdatePoint4 _wbp_point_prgress))
    (:5
      (Default|UpdatePoint5 _wbp_point_prgress)
      (CallFunction|TheMomentOfInfection))))

(fn UpdateTipsWidget
  (bind _returnvalue (Game|GetPlayerCameraManager 0))
  (bind _infectionprogressbar (Variables|Default|GetInfectionProgressBar))
  (bind _returnvalue_2 (Transformation|GetWorldLocation _infectionprogressbar))
  (bind _returnvalue_3 (Transformation|GetActorLocation _returnvalue))
  (bind _returnvalue_4 (Math|Rotator|FindLookatRotation _returnvalue_2 _returnvalue_3))
  (Transformation|SetWorldRotation _infectionprogressbar _returnvalue_4 false false)
  (Transformation|SetWorldRotation (Variables|Default|GetAlertProgressBar) _returnvalue_4 false false)
  (Transformation|SetWorldRotation (Variables|Default|GetAfterInfectionProgressBar) _returnvalue_4 false false)
  (Transformation|SetWorldRotation (Variables|Default|GetBubble) "0.000000,180.000000,0.000000" false false))

(fn InfectionProgressBarInit
  (bind _aswbp_point_prgress (Utilities|Casting|CastToWBP_PointPrgress (UserInterface|GetUserWidgetObject (Variables|Default|GetInfectionProgressBar))))
  (Variables|Default|SetWBP%20Point%20Prgress _aswbp_point_prgress)
  (bind _aswbp_npcafter_infection (Utilities|Casting|CastToWBP_NPCAfterInfection (UserInterface|GetUserWidgetObject (Variables|Default|GetAfterInfectionProgressBar))))
  (Variables|Default|SetWBP%20NPCAfter%20Infection _aswbp_npcafter_infection)
  (Rendering|SetVisibility (Variables|Default|GetAfterInfectionProgressBar) false false))

(fn ExpressionComponentInit
  (bind _aswbp_face_expression_npc (Utilities|Casting|CastToWBP_FaceExpression_Npc (UserInterface|GetUserWidgetObject (Variables|Default|GetExpressionComponent))))
  (bind _output_get (Variables|Default|SetWBP%20Face%20Expression%20Npc _aswbp_face_expression_npc))
  (Default|UpdateExpressionBrush _output_get (.OutItem (Utilities|Array|Random (Variables|Expression|GetDefault%20Expression)))))

(fn AlertProgressBarInit
  (bind _alertprogressbar (Variables|Default|GetAlertProgressBar))
  (Variables|Default|SetWBP%20NPCPatrol (.AsWBP%20NPCPatrol (Utilities|Casting|CastToWBP_NPCPatrol (UserInterface|GetUserWidgetObject _alertprogressbar))))
  (Rendering|SetVisibility _alertprogressbar false false)
  (Rendering|SetVisibility (Variables|Default|GetBubble) true false))

(fn SpotPlayer
  (CallFunction|UpdateExpression (.OutItem (Utilities|Array|Random (Variables|Expression|GetAngey%20Expression))) (Variables|Expression|GetAngey%20Skin))
  (Rendering|SetVisibility (Variables|Default|GetAlertProgressBar) true false)
  (Rendering|SetVisibility (Variables|Default|GetBubble) false false)
  (if (not (Variables|Patrol|GetbInGracePeriod))
    (Variables|Patrol|SetbInGracePeriod true)))

(fn AlertProgressBarReset
  (Progress|SetPercent (Variables|/Game/A_KOS/UI/SubWidgets/WBP_NPCPatrol.WBP_NPCPatrol_C|GetProgressBar (Variables|Default|GetWBP%20NPCPatrol)) 0.0)
  (Rendering|SetVisibility (Variables|Default|GetAlertProgressBar) false false)
  (Rendering|SetVisibility (Variables|Default|GetBubble) true false)
  (Variables|Patrol|SetbInGracePeriod false))

(fn AlertProgressBarSet
  (Progress|SetPercent (Variables|/Game/A_KOS/UI/SubWidgets/WBP_NPCPatrol.WBP_NPCPatrol_C|GetProgressBar (Variables|Default|GetWBP%20NPCPatrol)) (Variables|Patrol|GetAlertProgress)))

(fn AlertValueDrops
  (bind _output_get (Variables|Patrol|SetAlertProgress (Math|Float|Clamp(Float) (- (Variables|Patrol|GetAlertProgress) (* (/ (Utilities|Time|GetWorldDeltaSeconds) 1e+01) (Variables|/Game/A_KOS/Gameplay/BP_KS_PlayerState.BP_KS_PlayerState_C|GetHide%20Speed (.AsBP%20KS%20Player%20State (Utilities|Casting|CastToBP_KS_PlayerState (Variables|/Script/Engine.Pawn|GetPlayerState (Variables|Default|GetPlayer))))))))))
  (Alert|AlertProgressBarSet)
  (if (== _output_get 0.0)
    (Variables|Patrol|SetbInGracePeriod false)))

(fn AlertLevelRising
  (Variables|Patrol|SetAlertProgress (Math|Float|Clamp(Float) (/ (+ (Variables|Patrol|GetAlertProgress) (Utilities|Time|GetWorldDeltaSeconds)) (Variables|Patrol|GetMaxAlertTime))))
  (Alert|AlertProgressBarSet))

(fn UpdateExpression
  (params (Expression :type Texture%202D%20Object%20Reference) (SkinMaterial :type Material%20Interface%20Object%20Reference))
  (Default|UpdateExpressionBrush (Variables|Default|GetWBP%20Face%20Expression%20Npc) Expression)
  (Rendering|Material|SetMaterial (Variables|Character|GetMesh) 0 SkinMaterial))

(fn UpdateBubble
  (Utilities|Time|ClearandInvalidateTimerbyHandle (Variables|Default|GetPlayableTimer))
  (Default|SetBubbleVisbility (Variables|Default|GetWBP%20NPCBubble) (.OutItem (Utilities|Array|Random (Variables|Default|GetBubbleTextArray))) "/Game/A_KOS/Asset/Textures/qi pao.qi pao" 1.0)
  (bind _returnvalue (Utilities|Time|SetTimerbyEvent (EventDispatchers|CreateEvent :!event CancelBubble) 4.0))
  (Variables|Default|SetPlayableTimer _returnvalue))

(fn CancelBubble
  (Default|SetBubbleHiden (Variables|Default|GetWBP%20NPCBubble)))

(fn TheMomentOfInfection
  (Rendering|SetVisibility (Variables|Default|GetInfectionProgressBar) false false)
  (Rendering|SetVisibility (Variables|Default|GetAfterInfectionProgressBar) true false)
  (AI|Components|Blackboard|SetValueasBool (AI|GetBlackboard 0) (Utilities|Name|MakeLiteralName "bEncounteredPlayer") false)
  (Alert|AlertProgressBarReset))

(fn InfectionFailure
  (Variables|Default|SetbInfection false)
  (Variables|Infection|SetInfection%20Value 0)
  (CallFunction|ChangeInfectionValue)
  (Progress|SetPercent (Variables|/Game/A_KOS/UI/SubWidgets/WBP_NPCAfterInfection.WBP_NPCAfterInfection_C|GetProgressBar (Variables|Default|GetWBP%20NPCAfter%20Infection)) 1.0)
  (Rendering|SetVisibility (Variables|Default|GetInfectionProgressBar) true false)
  (Rendering|SetVisibility (Variables|Default|GetAfterInfectionProgressBar) false false))

(fn CountdowntotheEndOfInfection
  (params (DeltaTime :type Float%20%28double-precision%29))
  (bind _wbp_npcafter_infection (Variables|Default|GetWBP%20NPCAfter%20Infection))
  (bind _countdown_infection_value (Variables|Infection|GetCountdown%20Infection%20Value))
  (bind _returnvalue (/ DeltaTime _countdown_infection_value))
  (bind _progressbar (Variables|/Game/A_KOS/UI/SubWidgets/WBP_NPCAfterInfection.WBP_NPCAfterInfection_C|GetProgressBar _wbp_npcafter_infection))
  (bind _percent (Variables|/Script/UMG.ProgressBar|GetPercent _progressbar))
  (bind _returnvalue_2 (- _percent _returnvalue))
  (bind _returnvalue_3 (Math|Float|Clamp(Float) _returnvalue_2))
  (Progress|SetPercent _progressbar _returnvalue_3)
  (if (== _returnvalue_3 0.0)
    (CallFunction|InfectionFailure)
    (Alert|AlertProgressBarReset)))

(fn Reinfection
  (Progress|SetPercent (Variables|/Game/A_KOS/UI/SubWidgets/WBP_NPCAfterInfection.WBP_NPCAfterInfection_C|GetProgressBar (Variables|Default|GetWBP%20NPCAfter%20Infection)) 1.0))