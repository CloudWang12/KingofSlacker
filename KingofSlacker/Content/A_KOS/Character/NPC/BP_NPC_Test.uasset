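; Test NPC Blueprint that can spot the player and be infected by projectile damage.
; BeginPlay sets up expression, infection and detection widgets; Tick turns the infection bar toward the camera.
; Vision overlap with BP_TestCharacter flags detection and reveals its bar, but progress and grace-period logic are stubs.
; Infection accumulates damage up to a maximum; a separate, locally uncalled function updates the five-point display, and debug readouts are disconnected.
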(event OnComponentBeginOverlap(Vision)
  (params (OverlappedComponent :type Primitive%20Component%20Object%20Reference) (OtherActor :type Actor%20Object%20Reference) (OtherComp :type Primitive%20Component%20Object%20Reference) (OtherBodyIndex :type Integer) (bFromSweep :type Boolean) (SweepResult :type Hit%20Result%20Structure%20%28by%20ref%29))
  ;[0.15 0.15 0.15 0.5] NPC发现玩家
  (bind _asbp_test_character (Utilities|Casting|CastToBP_TestCharacter OtherActor))
  (bind _output_get (Variables|Default|SetPlayer _asbp_test_character))
  (Development|PrintString (Utilities|String|Append (Utilities|GetDisplayName self) "看见了:" (Utilities|GetDisplayName _output_get)))
  (CallFunction|SpotPlayer))

(event Custom|UpdateDetectionProgress
  (if (Variables|Patrol|GetbIsPlayerDetected)
    _))

(event EventBeginPlay
  (CallFunction|ExpressionComponentInit)
  (CallFunction|InfectionProgressBarInit)
  (CallFunction|DetectionProgressBarInit))

(event Collision|EventActorBeginOverlap
  (params (OtherActor :type Actor%20Object%20Reference)))

(event EventTick
  (params (DeltaSeconds :type Float%20%28single-precision%29))
  (CallFunction|DEBUGALL DeltaSeconds)
  (CallFunction|UpdateTipsWidget))

(fn ConstructionScript)

(fn DEBUG
  (params (Append :type String) (Context :type String) (TextColor :type Linear%20Color%20Structure) (Duration :type Float%20%28single-precision%29))
  (Development|PrintString (Utilities|String|Append Append Context) true true TextColor Duration))

(fn DEBUGALL
  (params (Duration :type Float%20%28single-precision%29)))

(fn Infection
  (params (Projectile%20damage :type Integer))
  (if (< (Variables|Infection|GetInfection%20Value) (Variables|Infection|GetMax%20Infection%20Value))
    (if (< (+ Projectile%20damage (Variables|Infection|GetInfection%20Value)) (Variables|Infection|GetMax%20Infection%20Value))
      (Variables|Infection|SetInfection%20Value (+ Projectile%20damage (Variables|Infection|GetInfection%20Value)))
      (Development|PrintString (Utilities|String|Append "NPC:" (Utilities|GetDisplayName self) "的感染值:" (Utilities|String|ToString(Integer) (Variables|Infection|GetInfection%20Value))))
      (else
        (Variables|Infection|SetInfection%20Value (Variables|Infection|GetMax%20Infection%20Value) :!label _label)
        (Development|PrintString (Utilities|String|Append "NPC:" (Utilities|GetDisplayName self) "已被感染"))))
    (else
      (goto _label))))

(fn ChangeInfectionValue
  (bind _wbp_point_prgress (Variables|Default|GetWBP%20Point%20Prgress))
  (switch int (Variables|Infection|GetInfection%20Value)
    (:1
      (Default|UpdatePoint1 _wbp_point_prgress))
    (:2
      (Default|UpdatePoint2 _wbp_point_prgress))
    (:3
      (Default|UpdatePoint3 _wbp_point_prgress))
    (:4
      (Default|UpdatePoint4 _wbp_point_prgress))
    (:5
      (Default|UpdatePoint5 _wbp_point_prgress))))

(fn UpdateTipsWidget
  (bind _infectionprogressbar (Variables|Default|GetInfectionProgressBar))
  (Transformation|SetWorldRotation _infectionprogressbar (Math|Rotator|FindLookatRotation (Transformation|GetWorldLocation _infectionprogressbar) (Transformation|GetActorLocation (Game|GetPlayerCameraManager 0))) false false))

(fn InfectionProgressBarInit
  (bind _aswbp_point_prgress (Utilities|Casting|CastToWBP_PointPrgress (UserInterface|GetUserWidgetObject (Variables|Default|GetInfectionProgressBar))))
  (Variables|Default|SetWBP%20Point%20Prgress _aswbp_point_prgress))

(fn ExpressionComponentInit
  (bind _aswbp_face_expression (Utilities|Casting|CastToWBP_FaceExpression (UserInterface|GetUserWidgetObject (Variables|Default|GetExpressionComponent))))
  (bind _output_get (Variables|Default|SetWBP%20Face%20Expression _aswbp_face_expression))
  (Default|UpdateExpressionBrush _output_get (Variables|Default|GetDefault%20Expression)))

(fn DetectionProgressBarInit
  (Rendering|SetVisibility (Variables|Default|GetDetectionProgressBar) false false))

(fn SpotPlayer
  (Variables|Patrol|SetbIsPlayerDetected true)
  (Rendering|SetVisibility (Variables|Default|GetDetectionProgressBar) true false)
  (if (not (Variables|Patrol|GetbInGracePeriod))
    (Variables|Patrol|SetbInGracePeriod false)))