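; BP_SightSystem is an NPC vision-cone component for a BP_NPC_Test owner.
; Each tick it writes FOV, radius, observer position and direction to the MPC_NPCSight parameter collection for materials.
; It also fans Visibility line traces across the FOV and appends the hits to BaseHits.
; Drawing those hits as triangles into a render target is unfinished: the hit loop is empty and the canvas nodes are disconnected.
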(event EventBeginPlay
  (bind _asbp_npc_test (Utilities|Casting|CastToBP_NPC_Test (Components|GetOwner self)))
  (Variables|Default|SetBP%20NPC%20Test _asbp_npc_test)
  (Variables|Default|SetRT%20Half%20Size (Math|Conversions|ToFloat(Integer) (/ (Variables|/Script/Engine.TextureRenderTarget2D|GetSizeX (Variables|Default|GetRenderTarget)) 2))))

(event EventTick
  (params (DeltaSeconds :type Float%20%28single-precision%29))
  (Utilities|FlowControl|Sequence
    (:then_0
      (Rendering|Material|SetScalarParameterValue "/Game/A_KOS/Character/NPC/ShightSystem/Material/MPC_NPCSight.MPC_NPCSight" "FOV" (Variables|Default|GetHalfFOV) :!class /Script/Engine.KismetMaterialLibrary)
      (Rendering|Material|SetScalarParameterValue "/Game/A_KOS/Character/NPC/ShightSystem/Material/MPC_NPCSight.MPC_NPCSight" "SightRadius" (Variables|Default|GetSightRadius) :!class /Script/Engine.KismetMaterialLibrary)
      (Rendering|Material|SetVectorParameterValue "/Game/A_KOS/Character/NPC/ShightSystem/Material/MPC_NPCSight.MPC_NPCSight" "ObserverPosition" (Math|Conversions|ToLinearColor(Vector) (Transformation|GetWorldLocation)) :!class /Script/Engine.KismetMaterialLibrary)
      (Rendering|Material|SetVectorParameterValue "/Game/A_KOS/Character/NPC/ShightSystem/Material/MPC_NPCSight.MPC_NPCSight" "ObserverDirection" (Math|Conversions|ToLinearColor(Vector) (Math|Vector|GetForwardVector)) :!class /Script/Engine.KismetMaterialLibrary))
    (:then_1
      (CallFunction|DrawSightZone 1e+01))))

(fn DrawSightZone
  (params (Trace%20Draw%20Penetration%20Distance :type Float%20%28double-precision%29))
  (bind _returnvalue (Transformation|GetWorldLocation))
  (LocalVariables|SetBaseTraceSection (* (Math|Float|Truncate (/ (Variables|Default|GetHalfFOV) (Variables|Default|GetBaseTraceAngle))) 2))
  (Variables|Default|SetBaseTraceAngle (/ (* (Variables|Default|GetHalfFOV) 2.0) (LocalVariables|GetBaseTraceSection)))
  (Utilities|FlowControl|Sequence
    (:then_0
      (for _index (range 0 (LocalVariables|GetBaseTraceSection))
        (bind _outhit (Collision|LineTraceByChannel _returnvalue (+ _returnvalue (* (Math|Vector|GetForwardVector (Math|Rotator|MakeRotator 0.0 0.0 (+ (- (* _index (LocalVariables|GetBaseDeltaAngle)) (Variables|Default|GetHalfFOV)) (.yaw (Transformation|GetWorldRotation))))) (Variables|Default|GetSightRadius))) "TraceTypeQuery1" false 0 "None"))
        (Utilities|Array|Add (LocalVariables|GetBaseHits) _outhit)))
    (:then_1
      (for _index_2 (range 0 (- (Utilities|Array|LastIndex (LocalVariables|GetBaseHits)) 1))
        _))))