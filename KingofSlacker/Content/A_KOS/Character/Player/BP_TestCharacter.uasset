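; Player test character with a face-expression widget, swappable skin materials, proximity interaction and a throw-trajectory preview.
; BeginPlay caches controller, state and face widget, picks a random expression, binds status changes and opens a delayed tutorial tip.
; Sphere overlaps message interactable actors only in StationIdle; Tick debug-prints status and turns the tips toward the camera.
; The throw preview uses a looping timer to rebuild spline meshes along a predicted projectile path.
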(event OnComponentBeginOverlap(Sphere)
  (params (OverlappedComponent :type Primitive%20Component%20Object%20Reference) (OtherActor :type Actor%20Object%20Reference) (OtherComp :type Primitive%20Component%20Object%20Reference) (OtherBodyIndex :type Integer) (bFromSweep :type Boolean) (SweepResult :type Hit%20Result%20Structure%20%28by%20ref%29))
  (if (and (Utilities|DoesObjectImplementInterface OtherActor "/Script/KingofSlacker.InteractInterface") (Utilities|Enum|Equal(Enum) (Variables|/Game/A_KOS/Gameplay/BP_KS_PlayerState.BP_KS_PlayerState_C|GetPlayerStatus (Variables|Default|GetBP%20KS%20Player%20State)) "Station_Idle"))
    (Class|InteractInterface|Interact(Message) OtherActor true)))

(event OnComponentEndOverlap(Sphere)
  (params (OverlappedComponent :type Primitive%20Component%20Object%20Reference) (OtherActor :type Actor%20Object%20Reference) (OtherComp :type Primitive%20Component%20Object%20Reference) (OtherBodyIndex :type Integer))
  (if (and (Utilities|Enum|Equal(Enum) (Variables|/Game/A_KOS/Gameplay/BP_KS_PlayerState.BP_KS_PlayerState_C|GetPlayerStatus (Variables|Default|GetBP%20KS%20Player%20State)) "Station_Idle") (Utilities|DoesObjectImplementInterface OtherActor "/Script/KingofSlacker.InteractInterface"))
    (Class|InteractInterface|Interact(Message) OtherActor false)))

(event Custom|Draw%20Projectile%20Curve
  ;[0.15 0.15 0.15 0.5] 投掷物路线显示
  (bind _returnvalue (Utilities|Time|SetTimerbyEvent (delegate Custom|Update%20Projectile%20Curve) 0.01 true))
  (Variables|Default|SetProjectile%20Timer _returnvalue))

(event Custom|Update%20Projectile%20Curve
  (bind _projectile_spline (Variables|Default|GetProjectile%20Spline))
  ;[0.15 0.15 0.15 0.5] 投掷物路线显示
  (CallFunction|ClearSplinePoints)
  (bind _predictresult (Class|GameplayStatics|BlueprintPredictProjectilePathAdvanced (Utilities|Struct|MakePredictProjectilePathParams (Transformation|GetWorldLocation (Variables|Default|GetThrowPosition)) (+ (* (Variables|Default|GetThrow%20Force%20Forward) (Transformation|GetActorForwardVector)) (Math|Vector|MakeVector 0.0 0.0 (Variables|Default|GetThrow%20Force%20Up))) true 0.0 3.0 true "ECC_WorldDynamic" "ObjectTypeQuery1" (Utilities|Array|MakeArray self) 2e+01 0.0 "None" 0.0 false)))
  (for _array_element (.PathData (Utilities|Struct|BreakPredictProjectilePathResult _predictresult))
    (Spline|AddSplinePoint (Variables|Default|GetProjectile%20Spline) (.Location (Utilities|Struct|BreakPredictProjectilePathPointData _array_element)) "World" true))
  (for _index (range 3 (Spline|GetNumberOfSplinePoints (Variables|Default|GetProjectile%20Spline)))
    (bind _returnvalue (AddComponent|AddSplineMeshComponent true))
    (Utilities|Array|Add (Variables|Default|GetSpline%20Mesh) _returnvalue)
    (SplineMesh|SetStartandEnd _returnvalue (.Location (Spline|GetLocationandTangentatSplinePoint _projectile_spline _index "World")) (.Tangent (Spline|GetLocationandTangentatSplinePoint _projectile_spline _index "World")) (Math|Vector|Lerp(Vector) (.Location (Spline|GetLocationandTangentatSplinePoint _projectile_spline _index "World")) (.Location (Spline|GetLocationandTangentatSplinePoint _projectile_spline (+ _index 1) "World")) 0.5) (Math|Vector|Lerp(Vector) (.Tangent (Spline|GetLocationandTangentatSplinePoint _projectile_spline _index "World")) (.Tangent (Spline|GetLocationandTangentatSplinePoint _projectile_spline (+ _index 1) "World")) 0.5) true :!class /Script/Engine.SplineMeshComponent)))

(event Custom|Clear%20Spline%20Points
  (bind _spline_mesh (Variables|Default|GetSpline%20Mesh))
  ;[0.15 0.15 0.15 0.5] 投掷物路线显示
  (Components|DestroyComponent _spline_mesh)
  (Utilities|Array|Clear _spline_mesh)
  (Spline|ClearSplinePoints (Variables|Default|GetProjectile%20Spline) true))

(event EventBeginPlay
  (bind _asbp_ks_player_controller (Utilities|Casting|CastToBP_KS_PlayerController (Game|GetPlayerController 0)))
  (Variables|Default|SetBP%20KS%20Player%20Controller _asbp_ks_player_controller)
  (bind _asbp_ks_player_state (Utilities|Casting|CastToBP_KS_PlayerState (Game|GetPlayerState 0)))
  (Variables|Default|SetBP%20KS%20Player%20State _asbp_ks_player_state)
  (bind _aswbp_face_expression (Utilities|Casting|CastToWBP_FaceExpression (UserInterface|GetUserWidgetObject (Variables|Default|GetExpressionComponent))))
  (bind _output_get (Variables|Default|SetWBP%20Face%20Expression _aswbp_face_expression))
  (Default|UpdateExpressionBrush _output_get (.OutItem (Utilities|Array|Random (Variables|Default|GetDefault%20Expression))))
  (EventDispatchers|BindEventtoOnStatusChanged (Variables|Default|GetBP%20KS%20Player%20State) (EventDispatchers|CreateEvent :!event BindCharacterStatus))
  ;[0.15 0.15 0.15 0.5] 这里不需要用广播，做个延迟处理直接调用哪个新手引导教学就行了
  (Utilities|FlowControl|DoOnce false
    (:Completed
      (Utilities|FlowControl|Delay 1.0)
      (Default|OpenContentTips (Variables|/Game/A_KOS/Gameplay/BP_KS_PlayerController.BP_KS_PlayerController_C|GetOverlay (Variables|Default|GetBP%20KS%20Player%20Controller)) 1))))

(event EventTick
  (params (DeltaSeconds :type Float%20%28single-precision%29))
  (Development|PrintString (Utilities|String|EnumtoString (Variables|/Game/A_KOS/Gameplay/BP_KS_PlayerState.BP_KS_PlayerState_C|GetPlayerStatus (Variables|Default|GetBP%20KS%20Player%20State))) true true "(R=0.000000,G=0.660000,B=1.000000,A=1.000000)" DeltaSeconds)
  (CallFunction|UpdateTipsWidget))

(fn ConstructionScript)

(fn UpdateTipsWidget
  (bind _tips (Variables|Default|GetTips))
  (Transformation|SetWorldRotation _tips (Math|Rotator|FindLookatRotation (Transformation|GetWorldLocation _tips) (Transformation|GetActorLocation (Game|GetPlayerCameraManager 0))) false false))

(fn BindCharacterStatus
  (params (InStatus :type EPlayerStatus%20Enum :default "Player_Fishing"))
  (Variables|/Game/A_KOS/Gameplay/BP_KS_PlayerState.BP_KS_PlayerState_C|SetPlayerStatus (Variables|Default|GetBP%20KS%20Player%20State) InStatus))

(fn UpdateExpression
  (params (Expression :type Texture%202D%20Object%20Reference))
  (Default|UpdateExpressionBrush (Variables|Default|GetWBP%20Face%20Expression) Expression))

(fn InitializeCharacterOOTD
  (params (SkinIndex :type Integer))
  (Rendering|Material|SetMaterial (Variables|Character|GetMesh) 0 (Utilities|Array|Get(acopy) (Variables|Default|GetCharacterSkins) SkinIndex)))