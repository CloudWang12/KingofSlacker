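; Base player character that handles item interaction, cosmetics, throw aiming, area music and speed boosts.
; Sphere overlaps notify InteractInterface actors and bind item interactions, which update the tips widget and add wool income to PlayerState.
; A looping timer rebuilds the throw arc from predicted projectile paths as spline meshes, while BGM area overlaps switch tracks.
; Tick turns widgets toward the camera; helper functions set skin, expression, decoration, hat and operation guides.
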(event OnComponentBeginOverlap(Sphere)
  (params (OverlappedComponent :type Primitive%20Component%20Object%20Reference) (OtherActor :type Actor%20Object%20Reference) (OtherComp :type Primitive%20Component%20Object%20Reference) (OtherBodyIndex :type Integer) (bFromSweep :type Boolean) (SweepResult :type Hit%20Result%20Structure%20%28by%20ref%29))
  (if (Utilities|DoesObjectImplementInterface OtherActor "/Script/KingofSlacker.InteractInterface")
    (bind _output_get (Variables|Default|SetbInRange true))
    (Class|InteractInterface|Interact(Message) OtherActor _output_get)
    (bind _returnvalue (Class|InteractInterface|GetItemActorRef(Message) OtherActor))
    (Utilities|IsValid _returnvalue
      (:Is%20Valid
        (EventDispatchers|BindEventtoOnInteractItem _returnvalue (delegate Custom|InteractItem))))))

(event OnComponentEndOverlap(Sphere)
  (params (OverlappedComponent :type Primitive%20Component%20Object%20Reference) (OtherActor :type Actor%20Object%20Reference) (OtherComp :type Primitive%20Component%20Object%20Reference) (OtherBodyIndex :type Integer))
  (if (Utilities|DoesObjectImplementInterface OtherActor "/Script/KingofSlacker.InteractInterface")
    (bind _output_get (Variables|Default|SetbInRange false))
    (Class|InteractInterface|Interact(Message) OtherActor _output_get)))

(event OnComponentBeginOverlap(BGMBox)
  (params (OverlappedComponent :type Primitive%20Component%20Object%20Reference) (OtherActor :type Actor%20Object%20Reference) (OtherComp :type Primitive%20Component%20Object%20Reference) (OtherBodyIndex :type Integer) (bFromSweep :type Boolean) (SweepResult :type Hit%20Result%20Structure%20%28by%20ref%29))
  ;[0.15 0.15 0.15 0.5] BGM切换
  (bind _asbp_bgmarea (Utilities|Casting|CastToBP_BGMArea OtherActor))
  (if (not (== (Variables|/Game/A_KOS/Blueprints/Audio/BP_BGMArea.BP_BGMArea_C|GetBGMIndex _asbp_bgmarea) (Variables|Default|GetPrevious%20BGM)))
    (Variables|Default|SetPrevious%20BGM (Variables|/Game/A_KOS/Blueprints/Audio/BP_BGMArea.BP_BGMArea_C|GetBGMIndex _asbp_bgmarea))
    (Audio|Components|Audio|FadeOut (Variables|Default|GetBGM) 1.0 0.0 "Linear" :!class /Script/Engine.AudioComponent)
    (Audio|Components|Audio|SetSound (Variables|Default|GetBGM) (Utilities|Array|Get(acopy) (Variables|Default|GetBGMSound) (Variables|Default|GetPrevious%20BGM)))
    (Audio|Components|Audio|Play (Variables|Default|GetBGM) 0.0)))

(event Custom|Draw%20Projectile%20Curve
  ;[0.15 0.15 0.15 0.5] 投掷物路线显示
  (bind _returnvalue (Utilities|Time|SetTimerbyEvent (delegate Custom|Update%20Projectile%20Curve) 0.01 true))
  (Variables|Default|SetProjectile%20Timer _returnvalue))

(event Custom|Update%20Projectile%20Curve
  (bind _projectile_spline (Variables|Default|GetProjectile%20Spline))
  ;[0.15 0.15 0.15 0.5] 投掷物路线显示
  (CallFunction|ClearSplinePoints)
  (bind _predictresult (Class|GameplayStatics|BlueprintPredictProjectilePathAdvanced (Utilities|Struct|MakePredictProjectilePathParams (Transformation|GetWorldLocation (Variables|Default|GetThrowPosition)) (+ (* (Variables|Default|GetThrow%20Force%20Forward) (Transformation|GetActorForwardVector)) (Math|Vector|MakeVector 0.0 0.0 (Variables|Default|GetThrow%20Force%20Up))) true 0.0 3.0 true "ECC_WorldDynamic" "ObjectTypeQuery1" (Utilities|Array|MakeArray self) 2e+01 0.0 "None" 0.0 false)))
  (for _array_element (.PathData (Utilities|Struct|BreakPredictProjectilePathResult _predictresult))
    (Spline|AddSplinePoint (Variables|Default|GetProjectile%20Spline) (.Location (Utilities|Struct|BreakPredictProjectilePathPointData _array_element)) "World" true))
  (for _index (range 3 (Spline|GetNumberOfSplinePoints (Variables|Default|GetProjectile%20Spline)))
    (bind _returnvalue (AddComponent|AddSplineMeshComponent true))
    (Utilities|Array|Add (Variables|Default|GetSpline%20Mesh) _returnvalue)
    (SplineMesh|SetStartandEnd _returnvalue (.Location (Spline|GetLocationandTangentatSplinePoint _projectile_spline _index "World")) (.Tangent (Spline|GetLocationandTangentatSplinePoint _projectile_spline _index "World")) (Math|Vector|Lerp(Vector) (.Location (Spline|GetLocationandTangentatSplinePoint _projectile_spline _index "World")) (.Location (Spline|GetLocationandTangentatSplinePoint _projectile_spline (+ _index 1) "World")) 0.5) (Math|Vector|Lerp(Vector) (.Tangent (Spline|GetLocationandTangentatSplinePoint _projectile_spline _index "World")) (.Tangent (Spline|GetLocationandTangentatSplinePoint _projectile_spline (+ _index 1) "World")) 0.5) true :!class /Script/Engine.SplineMeshComponent)))

(event Custom|Clear%20Spline%20Points
  (bind _spline_mesh (Variables|Default|GetSpline%20Mesh))
  ;[0.15 0.15 0.15 0.5] 投掷物路线显示
  (Components|DestroyComponent _spline_mesh)
  (Utilities|Array|Clear _spline_mesh)
  (Spline|ClearSplinePoints (Variables|Default|GetProjectile%20Spline) true))

(event Custom|InteractItem
  (Utilities|FlowControl|Sequence
    (:then_0
      (Utilities|FlowControl|DoOnce false
        (:Completed
          (Default|OpenContentTips (Variables|/Game/A_KOS/Gameplay/BP_KS_PlayerController.BP_KS_PlayerController_C|GetOverlay (Variables|Default|GetBP%20KS%20Player%20Controller)) 7))))
    (:then_1
      _))
  (CallFunction|InitializeItemDef (stale OnComponentBeginOverlap(Sphere) _returnvalue)))

(event EventBeginPlay
  (Utilities|FlowControl|Sequence
    (:then_0
      (bind _asbp_ks_player_controller (Utilities|Casting|CastToBP_KS_PlayerController (Game|GetPlayerController 0)))
      (Variables|Default|SetBP%20KS%20Player%20Controller _asbp_ks_player_controller)
      (bind _asbp_ks_player_state (Utilities|Casting|CastToBP_KS_PlayerState (Game|GetPlayerState 0)))
      (Variables|Default|SetBP%20KS%20Player%20State _asbp_ks_player_state)
      (bind _aswbp_face_expression (Utilities|Casting|CastToWBP_FaceExpression (UserInterface|GetUserWidgetObject (Variables|Default|GetExpressionComponent))))
      (Variables|Default|SetWBP%20Face%20Expression _aswbp_face_expression)
      (bind _aswbp_character_tips (Utilities|Casting|CastToWBP_CharacterTips (UserInterface|GetUserWidgetObject (Variables|Default|GetTips))))
      (Variables|Default|SetWBP%20Character%20Tips _aswbp_character_tips)
      (bind _aswbp_operation_guide (Utilities|Casting|CastToWBP_OperationGuide (UserInterface|GetUserWidgetObject (Variables|Default|GetOperationGuide))))
      (Variables|Default|SetWBP%20Operation%20Guide _aswbp_operation_guide)
      (EventDispatchers|BindEventtoOnStatusChanged (Variables|Default|GetBP%20KS%20Player%20State) (EventDispatchers|CreateEvent :!event BindCharacterStatus))
      (Variables|/Game/A_KOS/Gameplay/BP_KS_PlayerState.BP_KS_PlayerState_C|SetPlayerStatus (Variables|Default|GetBP%20KS%20Player%20State) "Station_Idle")
      ;[0.15 0.15 0.15 0.5] 这里不需要用广播，做个延迟处理直接调用哪个新手引导教学就行了
      (Utilities|FlowControl|DoOnce false
        (:Completed
          (Utilities|FlowControl|Delay 1.0)
          (Default|OpenContentTips (Variables|/Game/A_KOS/Gameplay/BP_KS_PlayerController.BP_KS_PlayerController_C|GetOverlay (Variables|Default|GetBP%20KS%20Player%20Controller)) 1))))))

(event EventTick
  (params (DeltaSeconds :type Float%20%28single-precision%29))
  (Development|PrintString (Utilities|String|EnumtoString (Variables|/Game/A_KOS/Gameplay/BP_KS_PlayerState.BP_KS_PlayerState_C|GetPlayerStatus (Variables|Default|GetBP%20KS%20Player%20State))) true true "(R=0.000000,G=0.660000,B=1.000000,A=1.000000)" DeltaSeconds)
  (CallFunction|UpdateTipsWidget))

(fn ConstructionScript)

(fn UpdateTipsWidget
  (bind _returnvalue (Game|GetPlayerCameraManager 0))
  (bind _tips (Variables|Default|GetTips))
  (bind _returnvalue_2 (Transformation|GetActorLocation _returnvalue))
  (bind _returnvalue_3 (Transformation|GetWorldLocation _tips))
  (bind _returnvalue_4 (Math|Rotator|FindLookatRotation _returnvalue_3 _returnvalue_2))
  (Transformation|SetWorldRotation _tips _returnvalue_4 false false)
  (Transformation|SetWorldRotation (Variables|Default|GetOperationGuide) _returnvalue_4 false false))

(fn BindCharacterStatus
  (params (InStatus :type EPlayerStatus%20Enum :default "Player_Fishing"))
  (Variables|/Game/A_KOS/Gameplay/BP_KS_PlayerState.BP_KS_PlayerState_C|SetPlayerStatus (Variables|Default|GetBP%20KS%20Player%20State) InStatus))

(fn UpdateExpression
  (params (Expression :type Texture%202D%20Object%20Reference))
  (Default|UpdateExpressionBrush (Variables|Default|GetWBP%20Face%20Expression) Expression))

(fn InitializeCharacterOOTD
  (params (SkinIndex :type Integer) (EmojiIndex :type Integer) (DecorationIndex :type Integer))
  (bind _decoration (Variables|Default|GetDecoration))
  (Rendering|Material|SetMaterial (Variables|Character|GetMesh) 0 (Utilities|Array|Get(acopy) (Variables|DecorationSystem|GetCharacterSkins) SkinIndex))
  (Default|UpdateExpressionBrush (Variables|Default|GetWBP%20Face%20Expression) (Utilities|Array|Get(acopy) (Variables|DecorationSystem|GetCharacterEmoji) EmojiIndex))
  (Components|StaticMesh|SetStaticMesh _decoration (Utilities|Array|Get(acopy) (Variables|DecorationSystem|GetCharactterDecoration) DecorationIndex))
  (Transformation|AttachComponentToComponent _decoration (Variables|Character|GetMesh) (Utilities|Select :Index DecorationIndex :Option%200 "" :Option%201 "Glasses" :Option%202 "Neck" :Option%203 "Watch") "KeepRelative" "KeepRelative" "KeepRelative" true))

(fn UpdateEquipment
  (params (ID :type Integer))
  (bind _datatable (Variables|Default|GetDataTable))
  (bind _outrownames (DataTable|GetDataTableRowNames _datatable))
  (for _array_element _outrownames
    (bind _returnvalue (Utilities|GetDataTableRow _datatable _array_element)
      (:then
        (if (== (.ItemID (Utilities|Struct|BreakItemType _returnvalue)) ID)
          (Utilities|IsValid (.ItemMesh (Utilities|Struct|BreakItemType _returnvalue))
            (:Is%20Valid
              (Components|StaticMesh|SetStaticMesh (Variables|Default|GetHat) (.ItemMesh (Utilities|Struct|BreakItemType _returnvalue))))))))))

(fn InitializeItemDef
  (params (ItemRef :type Object%20Object%20Reference))
  (bind _returnvalue (Class|InteractInterface|GetTexture(Message) ItemRef))
  (bind _returnvalue_2 (Class|InteractInterface|GetName(Message) ItemRef))
  (bind _returnvalue_3 (Class|InteractInterface|GetItemIncome(Message) ItemRef))
  (bind _returnvalue_4 (Class|InteractInterface|GetItemName(Message) ItemRef))
  (Default|UpdateCharacterTips (Variables|Default|GetWBP%20Character%20Tips) _returnvalue (Utilities|Text|ToText(Integer) _returnvalue_3) _returnvalue_2 _returnvalue_4)
  (Default|AddupWoolIncome (Variables|Default|GetBP%20KS%20Player%20State) _returnvalue_3))

(fn ShowOperationGuide
  (params (Index :type Integer))
  (Default|UpdateSwitcher (Variables|Default|GetWBP%20Operation%20Guide) Index)
  (Rendering|SetVisibility (Variables|Default|GetOperationGuide) true false))

(fn HideOperationGuide
  (params (Index :type Integer))
  (switch int Index
    (:0
      (if (Variables|Default|GetbInRange)
        (CallFunction|ShowOperationGuide 1)
        (else
          (Rendering|SetVisibility (Variables|Default|GetOperationGuide) false false))))
    (:1
      (if (and (not (Variables|Default|GetbInRange)) (Utilities|Enum|Equal(Enum) (Variables|/Game/A_KOS/Gameplay/BP_KS_PlayerState.BP_KS_PlayerState_C|GetPlayerStatus (Variables|Default|GetBP%20KS%20Player%20State)) "Station_Throwing"))
        (CallFunction|ShowOperationGuide)
        (else
          (Rendering|SetVisibility (Variables|Default|GetOperationGuide) false false))))))

(fn SpeedUp
  (bind _bp_ks_player_state (Variables|Default|GetBP%20KS%20Player%20State))
  (Variables|/Script/Engine.CharacterMovementComponent|SetMaxWalkSpeed (Variables|Character|GetCharacterMovement) (* (Variables|/Game/A_KOS/Gameplay/BP_KS_PlayerState.BP_KS_PlayerState_C|GetWalk%20Speed (Variables|Default|GetBP%20KS%20Player%20State)) 1.4))
  (Variables|/Game/A_KOS/Gameplay/BP_KS_PlayerState.BP_KS_PlayerState_C|SetThrow%20Aim%20Walk%20Speed _bp_ks_player_state (* (Variables|/Game/A_KOS/Gameplay/BP_KS_PlayerState.BP_KS_PlayerState_C|GetThrow%20Aim%20Walk%20Speed _bp_ks_player_state) 1.4)))

(fn SpeedReset
  (bind _bp_ks_player_state (Variables|Default|GetBP%20KS%20Player%20State))
  (Variables|/Script/Engine.CharacterMovementComponent|SetMaxWalkSpeed (Variables|Character|GetCharacterMovement) (Variables|/Game/A_KOS/Gameplay/BP_KS_PlayerState.BP_KS_PlayerState_C|GetWalk%20Speed (Variables|Default|GetBP%20KS%20Player%20State)))
  (Variables|/Game/A_KOS/Gameplay/BP_KS_PlayerState.BP_KS_PlayerState_C|SetThrow%20Aim%20Walk%20Speed _bp_ks_player_state (/ (Variables|/Game/A_KOS/Gameplay/BP_KS_PlayerState.BP_KS_PlayerState_C|GetThrow%20Aim%20Walk%20Speed _bp_ks_player_state) 1.4)))

(fn HiddenUp
  (bind _bp_ks_player_state (Variables|Default|GetBP%20KS%20Player%20State))
  (Variables|/Game/A_KOS/Gameplay/BP_KS_PlayerState.BP_KS_PlayerState_C|SetHide%20Speed _bp_ks_player_state (* (Variables|/Game/A_KOS/Gameplay/BP_KS_PlayerState.BP_KS_PlayerState_C|GetHide%20Speed _bp_ks_player_state) 1.2)))

(fn HiddenReset
  (bind _bp_ks_player_state (Variables|Default|GetBP%20KS%20Player%20State))
  (Variables|/Game/A_KOS/Gameplay/BP_KS_PlayerState.BP_KS_PlayerState_C|SetHide%20Speed _bp_ks_player_state (/ (Variables|/Game/A_KOS/Gameplay/BP_KS_PlayerState.BP_KS_PlayerState_C|GetHide%20Speed _bp_ks_player_state) 1.2)))